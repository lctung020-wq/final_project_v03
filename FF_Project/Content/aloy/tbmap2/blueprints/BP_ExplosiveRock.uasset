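; BP_ExplosiveRock is a rock actor that bursts into fire when it hits a Character.
; On BeginPlay it hides itself and disables collision, then becomes visible and collidable after a fixed delay.
; A Character hit spawns a fire emitter and plays a sound at the saved hit location, then destroys the rock after a short delay.
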(event EventBeginPlay
  (Rendering|SetActorHiddenInGame true)
  (Collision|SetActorEnableCollision false)
  (Utilities|FlowControl|Delay 1e+01)
  (Development|PrintString "rockplay")
  (Rendering|SetActorHiddenInGame false)
  (Collision|SetActorEnableCollision true))

(event Collision|EventActorBeginOverlap
  (params (OtherActor :type Actor%20Object%20Reference)))

(event EventTick
  (params (DeltaSeconds :type Float%20%28single-precision%29)))

(event Collision|EventHit
  (params (MyComp :type Primitive%20Component%20Object%20Reference) (Other :type Actor%20Object%20Reference) (OtherComp :type Primitive%20Component%20Object%20Reference) (bSelfMoved :type Boolean) (HitLocation :type Vector :default "0, 0, 0") (HitNormal :type Vector :default "0, 0, 0") (NormalImpulse :type Vector :default "0, 0, 0") (Hit :type Hit%20Result%20Structure%20%28by%20ref%29))
  (Variables|Default|SetSavedHitLocation HitLocation)
  (Utilities|Casting|CastToCharacter Other)
  (Effects|SpawnEmitteratLocation "/Game/aloy/maps/TemplesOfCambodia/Demo/EpicContent/StarterContent/Particles/P_Fire.P_Fire" (Variables|Default|GetSavedHitLocation))
  (Audio|PlaySoundatLocation "/Engine/EditorSounds/GamePreview/StartPlayInEditor.StartPlayInEditor" (Variables|Default|GetSavedHitLocation) "0, 0, 0" 1.0 1.0 0.0 0 0 0 0)
  (Utilities|FlowControl|Delay 0.5)
  (Actor|DestroyActor)
  (Development|PrintString "Destroy"))

(fn ConstructionScript)