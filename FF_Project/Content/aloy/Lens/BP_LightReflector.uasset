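; BP_LightReflector is a reflector actor that toggles its SpotLight based on line-trace hits against other BP_LightReflector actors.
; Each Tick it runs a debug-drawn visibility trace toward a point built from its forward vector alone, without adding actor location.
; On a reflector hit, it switches off the previously stored reflector, stores the new one and turns on its own light.
; A miss leaves lights unchanged.
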(event Custom|lightoff
  (Rendering|SetVisibility (Variables|Default|GetSpot%20Light) false false))

(event Custom|lighton
  (Rendering|SetVisibility (Variables|Default|GetSpot%20Light) true false))

(event EventTick
  (params (DeltaSeconds :type Float%20%28single-precision%29))
  (bind _returnvalue (Transformation|GetActorForwardVector))
  ;[1 1 1] Line Trace
  (bind (_outhit _returnvalue_2) (Collision|LineTraceByChannel (Transformation|GetActorLocation) (+ (* _returnvalue 2e+03) _returnvalue) "TraceTypeQuery1" false 0 "ForOneFrame" false))
  (if _returnvalue_2
    (bind _asbp_light_reflector (Utilities|Casting|CastToBP_LightReflector (.HitActor (Collision|BreakHitResult _outhit))))
    (Utilities|IsValid (Variables|Default|GetLastHitLight)
      (:Is%20Valid
        (CallFunction|Lightoff (stale _output_get)))
      (:Is%20Not%20Valid
        _))
    (bind _output_get (Variables|Default|SetLastHitLight _asbp_light_reflector))
    (CallFunction|Lighton)))

(event Collision|EventActorBeginOverlap
  (params (OtherActor :type Actor%20Object%20Reference)))

(event EventBeginPlay)

(fn ConstructionScript)