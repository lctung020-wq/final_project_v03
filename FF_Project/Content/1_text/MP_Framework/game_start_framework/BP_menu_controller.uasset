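; Player controller for the multiplayer menu and lobby, handling UI input and the lobby widget on the client.
; On BeginPlay the local controller shows the cursor and switches to UI-only input.
; Events create and show the lobby menu, then pass start-button readiness and player-count status to it, with comments noting they should run on the owning client.
; Ending a client session destroys it and opens the main menu map.
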(event Custom|EndClientSession
  (|DestroySession self
    (:then
      (Game|OpenLevel(byName) "MainMenu_Map"))))

(event Custom|create_Lobby_menu
  ;[0.06555 0.06715 0.15 0.5 45] lobby menu UMG
  ;;[0.15 0.15 0.15 0.5] need to make sure is replicates to owning client
  (CallFunction|UiShowLobbyMenu))

(event Custom|updat%20player%20statys%20text
  (params (CurrentPlayers :type Integer))
  ;[0.06555 0.06715 0.15 0.5 45] lobby menu UMG
  (Default|UpdatePlayerStatusText (Variables|Default|GetUMG_lobby%20menu) CurrentPlayers))

(event Custom|Client_RefreshStartButton
  (params (butt_is%20ready :type Boolean))
  (bind _umg_lobby_menu (Variables|Default|GetUMG_lobby%20menu))
  ;[0.06555 0.06715 0.15 0.5 45] lobby menu UMG
  ;;[0.15 0.15 0.15 0.5] UI 只能在客戶端被操控, so is run on owning client
  (Utilities|IsValid _umg_lobby_menu
    (:Is%20Valid
      (Default|UpdateStartButton _umg_lobby_menu butt_is%20ready))))

(event EventBeginPlay
  ;[0.15 0.15 0.15 0.5] set input mode UI only
  (if (Pawn|IsLocalController)
    (Variables|Default|SetbShowMouseCursor true)
    (Input|SetInputModeUIOnly self 0 "DoNotLock" false)))

(fn ConstructionScript)

(fn UiShowLobbyMenu
  (Utilities|IsValid 0
    (:Is%20Valid
      _)
    (:Is%20Not%20Valid
      (bind _returnvalue (UserInterface|CreateWidget "/Game/1_text/MP_Framework/game_start_framework/game_start_UI/UWG_LobbyMenu.UWG_LobbyMenu_C" self))
      (Variables|Default|SetUMG_lobby%20menu _returnvalue)))
  (UserInterface|Viewport|AddtoViewport (Variables|Default|GetUMG_lobby%20menu) 0)
  (return))

(fn OnRepMyStatusText)