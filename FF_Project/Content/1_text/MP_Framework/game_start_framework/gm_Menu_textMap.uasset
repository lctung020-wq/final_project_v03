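; Menu game mode that sets up the multiplayer lobby as players join.
; On the lobby map, HandleStartingNewPlayer stores each BP_menu_controller and has it create its lobby menu.
; The server then refreshes the first player's start button, marking it ready at two or more players.
; Every stored controller also gets the updated player count for its status text, with debug prints along the way.
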(event Custom|CheckLobbyPlayerCount
  (Variables|Default|Sethost%20is%20ready (>= (Utilities|Array|Length (Variables|Default|GetAll_connerted%20Player)) 2))
  (if (Networking|IsServer)
    (Default|ClientRefreshStartButton (Utilities|Array|Get(acopy) (Variables|Default|GetAll_connerted%20Player)) (Variables|Default|Gethost%20is%20ready))))

(event Custom|check%20is%20player%20join?
  (params (joiningPlayer :type Player%20Controller%20Object%20Reference))
  (bind _all_connerted_player (Variables|Default|GetAll_connerted%20Player))
  (bind _returnvalue (Utilities|Array|Length _all_connerted_player))
  (Utilities|Casting|CastToBP_menu_controller joiningPlayer
    (:then
      (for _array_element _all_connerted_player
        (Development|PrintString (Utilities|String|ToString(Integer) _returnvalue) true true "(R=0.000000,G=0.660000,B=1.000000,A=1.000000)" 1e+01)
        (Default|UpdatPlayerStatysText _array_element _returnvalue)))
    (:CastFailed
      (Development|PrintString "failed at check is player join?_gm_menu"))))

(event EventBeginPlay)

(event EventTick
  (params (DeltaSeconds :type Float%20%28single-precision%29)))

(event EventHandleStartingNewPlayer
  (params (NewPlayer :type Player%20Controller%20Object%20Reference))
  ;[0.15 0.15 0.15 0.5] gets executed if a new player enters the session and this will return a player controller
  ;[0.15 0.15 0.15 0.5] maybe need execute this game mode in something like upgrade menu
  (bind _returnvalue (Game|GetCurrentLevelName true))
  (switch string _returnvalue
    (:lobby_menu_map_text
      (bind _asbp_menu_controller (Utilities|Casting|CastToBP_menu_controller NewPlayer))
      (Utilities|Array|Add (Variables|Default|GetAll_connerted%20Player) _asbp_menu_controller)
      (Default|CreateLobbyMenu _asbp_menu_controller)
      (CallFunction|CheckLobbyPlayerCount)
      (CallFunction|CheckIsPlayerJoin? _asbp_menu_controller))))

(fn ConstructionScript)