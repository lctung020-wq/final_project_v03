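; BP_QTE_agency is a trigger actor that notifies a character's controller of a quick-time event when the character overlaps its sphere.
; Only the server acts on the overlap, reading the current QTE state from the gm_play_map game mode.
; In either of the first two states it sends QteCatchCtrlMessage to the controller, passing the game mode.
; Several older controller-registration and QTE-start chains remain disconnected, alongside debug prints.
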(event OnComponentBeginOverlap(Spherecoll)
  (params (OverlappedComponent :type Primitive%20Component%20Object%20Reference) (OtherActor :type Actor%20Object%20Reference) (OtherComp :type Primitive%20Component%20Object%20Reference) (OtherBodyIndex :type Integer) (bFromSweep :type Boolean) (SweepResult :type Hit%20Result%20Structure%20%28by%20ref%29))
  (Networking|SwitchHasAuthority
    (:Authority
      (Development|PrintString "BP_QTE_agency:is Authority       g4d" true true "(R=0.000000,G=0.660000,B=1.000000,A=1.000000)" 1e+01)
      (bind _ascharacter (Utilities|Casting|CastToCharacter OtherActor))
      (Development|PrintString (Utilities|GetDisplayName (Pawn|GetController _ascharacter)))
      (bind _asgm_play_map (Utilities|Casting|CastTogm_play_map (Game|GetGameMode)))
      (if (Utilities|Enum|Equal(Enum) (Variables|/Game/1_text/MP_Framework/game_play_framework/gm_play_map.gm_play_map_C|GetcurrentQTEStste _asgm_play_map) "NewEnumerator0")
        (Class|BPIOrgan|QteCatchCtrl(Message) (Pawn|GetController _ascharacter) _asgm_play_map)
        (elif (Utilities|Enum|Equal(Enum) (Variables|/Game/1_text/MP_Framework/game_play_framework/gm_play_map.gm_play_map_C|GetcurrentQTEStste _asgm_play_map) "NewEnumerator1")
          (Class|BPIOrgan|QteCatchCtrl(Message) (Pawn|GetController _ascharacter) _asgm_play_map))))
    (:Remote
      (Development|PrintString "BP_QTE_agency:is remote      g4d" true true "(R=0.000000,G=1.000000,B=0.116009,A=1.000000)" 1e+01))))

(event Custom|rest
  (Utilities|FlowControl|DoOnce false) ; enters at Reset
)

(event EventBeginPlay)

(event Collision|EventActorBeginOverlap
  (params (OtherActor :type Actor%20Object%20Reference)))

(event EventTick
  (params (DeltaSeconds :type Float%20%28single-precision%29)))

(fn ConstructionScript)