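; Multiplayer player controller for a cooperative QTE, also hosting subtitle and boss health UI and an authority-checked damage relay.
; It forwards QTE requests to gm_play_map, whose state enum decides between calling the partner for help and adding clamped click energy.
; CLN-prefixed events manage waiting, help and QTE widgets through a reuse-or-create helper, updating fill and playing success or fail animations.
; Debug prints and disconnected older QTE timer logic remain.
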(event Custom|CLN_umg%20boss%20hp
  (params (TargetManager :type BP%20Boss%20Fight%20Manager%20Gv%2002%20Object%20Reference))
  ;[0.15 0.15 0.15 0.5 173] Boss
  (bind _returnvalue (UserInterface|CreateWidget "/Game/Test/WBP_BossHPBar_g02.WBP_BossHPBar_g02_C" 0 TargetManager 0))
  (bind _output_get (Variables|Default|Setas%20WBP_BossHPBar _returnvalue))
  (UserInterface|Viewport|AddtoViewport _returnvalue 0)
  (Actor|GetActorOfClass "/Game/Test/BP_BossFightManager_Gv02.BP_BossFightManager_Gv02_C"))

(event Custom|ser%20remove%20all%20player%20ctrl
  ;[0.15 0.15 0.15 0.5 263] QTE
  (bind _asgm_play_map (Utilities|Casting|CastTogm_play_map (Game|GetGameMode)))
  (Variables|/Game/1_text/MP_Framework/game_play_framework/gm_play_map.gm_play_map_C|Setall_Qte%20Triger%20Controller _asgm_play_map (Utilities|Array|MakeArray 0)))

(event Custom|QTE_fail
  (bind _as_qte_switch_uwg_1 (Variables|QTE|GetAs%20QTE%20Switch%20UWG%201))
  (bind _fail (Variables|/Game/1_text/MP_Framework/game_play_framework/QTE/QTE_UI/QTE_Switch_UWG.QTE_Switch_UWG_C|Getfail _as_qte_switch_uwg_1))
  ;[0.03925 0.15 0.1345 0.5] QTE_fail
  (Utilities|Time|PauseTimerbyHandle (Variables|QTE|Getqte%20TIMER%20handle))
  (UserInterface|Animation|PlayAnimation _as_qte_switch_uwg_1 _fail 0.0 1 "Forward" 1.0 false)
  (Class|UserWidget|BindtoAnimationFinished (Variables|QTE|GetAs%20QTE%20Switch%20UWG%201) _fail (delegate Custom|Hide_umg)))

(event Custom|CLN_creat%20start_QTE
  (params (player%20ctrl :type BP%20Player%20Controller%20Text%20Object%20Reference))
  ;[0.15 0.15 0.15 0.5 263] QTE
  ;;[0.15 0.15 0.15 0.5] creat start qte UI
  (CallFunction|RemovefromParentinCtrl)
  (bind _uiwidget (CallFunction|CreateWidget "/Game/1_text/MP_Framework/game_play_framework/QTE/QTE_UI/QTE_Switch_UWG.QTE_Switch_UWG_C" false (Variables|Default|GetUMG_qte%20switch)))
  (Variables|Default|SetUMG_qte%20switch _uiwidget)
  (bind _asqte_switch_uwg (Utilities|Casting|CastToQTE_Switch_UWG _uiwidget)
    (:then
      (Variables|QTE|SetAs%20QTE%20Switch%20UWG%201 _asqte_switch_uwg))
    (:CastFailed
      (Development|PrintString "Qte switch ui cast failed        a7f75ag74s74ssss" true true "(R=1.000000,G=0.104708,B=0.000000,A=1.000000)" 1e+01))))

(event Custom|CLN_update%20QTE
  (params (player%200%25 :type Float%20%28double-precision%29) (player1%25 :type Float%20%28double-precision%29))
  (Default|SetFill (Variables|QTE|GetAs%20QTE%20Switch%20UWG%201) player%200%25 player1%25))

(event Custom|CC_UMG_show
  (bind _returnvalue (UserInterface|CreateWidget "/Game/1_text/UI/CC/W_CC.W_CC_C" self))
  (bind _output_get (Variables|cc_umg|Setumg_cc _returnvalue))
  (UserInterface|Viewport|AddtoViewport _output_get 0))

(event Custom|have%20damage
  (params (DamagedActor :type Actor%20Object%20Reference) (BaseDamage :type Float%20%28single-precision%29) (EventInstigator :type Controller%20Object%20Reference) (DamageCauser :type Actor%20Object%20Reference))
  ;[0.15 0.15 0.15 0.5 173] Boss
  (Development|PrintString "fps player 1: on hit call 2                           sd54g45h")
  (Networking|SwitchHasAuthority
    (:Authority
      (Game|Damage|ApplyDamage DamagedActor BaseDamage EventInstigator DamageCauser)
      (Development|PrintString "ply_ctrl    have damage is call authority                7ty6ws4r"))
    (:Remote
      (Development|PrintString "ply_ctrl    have damage is call remote                7ty6ws4r"))))

(event Custom|CLN_updathp
  (params (max%20health :type Float%20%28double-precision%29) (health :type Float%20%28double-precision%29))
  (bind _as_wbp_bosshpbar (Variables|Default|Getas%20WBP_BossHPBar))
  ;[0.15 0.15 0.15 0.5 173] Boss
  (Development|PrintString (Utilities|String|Append "CLN_updathp boss hp is :" (Utilities|String|ToString(Float) health)) true true "(R=1.000000,G=0.081181,B=0.000000,A=1.000000)")
  (Utilities|IsValid _as_wbp_bosshpbar
    (:Is%20Valid
      (Default|UMGUpdateHP _as_wbp_bosshpbar health max%20health)
      (Development|PrintString "fps player 1: on hit call 6                           sd54g45h"))))

(event Custom|SER_umg%20boss%20hp
  (params (TargetManager :type BP%20Boss%20Fight%20Manager%20Gv%2002%20Object%20Reference))
  ;[0.15 0.15 0.15 0.5 173] Boss
  (CallFunction|CLNUmgBossHp TargetManager))

(event Custom|call%20other%20player
  (params (calling%20help%20controller :type Player%20Controller%20Object%20Reference))
  ;[0.15 0.15 0.15 0.5 263] QTE
  ;;[0.15 0.15 0.15 0.5 28] call other to help_find out who need help
  (if (Utilities|IsValid (Variables|QTE|GetUMG_QTE_waiting))
    (Utilities|IsValid (Variables|QTE|GetUMG_call_player_help)
      (:Is%20Valid
        (Development|PrintString "call other player valid _true    5413654"))
      (:Is%20Not%20Valid
        (Development|PrintString "call other player valid _false    5413654")
        (CallFunction|SRVNotifyOtherPlayer calling%20help%20controller)
        (Development|PrintString "playerB_is call")))
    (else
      (Development|PrintString "Is  waiting other_player_UWG Valid? is false         zfvz5"))))

(event Custom|QTE%20_DecayRate
  ;[0.15 0.15 0.15 0.5 263] QTE
  (Variables|QTE|SetQTE%20CurrentEnergy (- (Variables|QTE|GetQTE%20CurrentEnergy) (* (Variables|QTE|GetQTE%20DecayRate) (Utilities|Time|GetWorldDeltaSeconds))))
  (Development|PrintString "QTE _DecayRate is call          35fv35a6szvg45sbh4xc" true true "(R=0.360498,G=0.869700,B=1.000000,A=1.000000)"))

(event Custom|CNL%20updat%20qte
  (params (%25_player1 :type Float%20%28single-precision%29) (%25_player2 :type Float%20%28single-precision%29))
  (bind _as_qte_switch_uwg_1 (Variables|QTE|GetAs%20QTE%20Switch%20UWG%201))
  ;[0.15 0.15 0.15 0.5 263] QTE
  (Default|SetFill _as_qte_switch_uwg_1 %25_player1 %25_player2)
  (Default|PlayerPulse _as_qte_switch_uwg_1))

(event Custom|SRV_show%20_Start_QTE
  (Utilities|Casting|CastTogm_play_map (Game|GetGameMode)))

(event Custom|CLN_showWaitingUI
  (params (remove%20ui? :type Boolean))
  ;[0.15 0.15 0.15 0.5 263] QTE
  ;;[0.15 0.15 0.15 0.5] create call help_waiting_UMG
  (bind _uiwidget (CallFunction|CreateWidget "/Game/1_text/MP_Framework/game_play_framework/QTE/QTE_UI/QTE_waiting__other_player.QTE_waiting__other_player_C" false (Variables|QTE|GetUMG_QTE_waiting)))
  (bind _output_get (Variables|QTE|SetUMG_QTE_waiting _uiwidget))
  (Utilities|IsValid _output_get
    (:Is%20Valid
      (Development|PrintString "UMG_QTE_waiting is valid"))
    (:Is%20Not%20Valid
      (Development|PrintString "UMG_QTE_waiting is valid" true true "(R=1.000000,G=0.019225,B=0.000000,A=1.000000)"))))

(event Custom|ser%20_Spawn%20Sound%20at%20Location
  (params (Sound :type Sound%20Base%20Object%20Reference))
  ;[0.15 0.15 0.15 0.5 263] QTE
  (Audio|SpawnSoundatLocation Sound "0, 0, 0" "0, 0, 0" 1.0 1.0 0.0 0 0))

(event Custom|ser%20call%20gm
  ;[0.15 0.15 0.15 0.5 263] QTE
  (Development|PrintString "ser call gm is be call         5af4a6aasdf")
  (bind _asgm_play_map (Utilities|Casting|CastTogm_play_map (Game|GetGameMode)))
  (Variables|Default|SetAs%20Gm%20Play%20Map _asgm_play_map)
  (if (Utilities|Enum|Equal(Enum) (Variables|/Game/1_text/MP_Framework/game_play_framework/gm_play_map.gm_play_map_C|GetcurrentQTEStste (Variables|Default|GetAs%20Gm%20Play%20Map)) "NewEnumerator0")
    (Default|SERWaitingQTE (Variables|Default|GetAs%20Gm%20Play%20Map) self)
    (Development|PrintString "QTE_agency_calling sRV start QTe done")))

(event Custom|remove%20QTE%20switch%20umg
  ;[0.15 0.15 0.15 0.5 263] QTE
  ;;[0.15 0.15 0.15 0.5] remove QTE switch umg
  (Utilities|IsValid (Variables|Default|GetUMG_qte%20switch)
    (:Is%20Valid
      (Widget|RemovefromParent (Variables|Default|GetUMG_qte%20switch))
      (Development|PrintString "remove done_14455" true true "(R=0.368149,G=0.076611,B=1.000000,A=1.000000)" 5.0)
      (Variables|Default|SetUMG_qte%20switch 0)
      (Variables|QTE|SetAs%20QTE%20Switch%20UWG%201 0))
    (:Is%20Not%20Valid
      (Development|PrintString "umg is not valid(done remove)_14455" true true "(R=0.251143,G=0.000000,B=1.000000,A=1.000000)" 5.0))))

(event Custom|Remove%20from%20parent%20in%20ctrl
  ;[0.15 0.15 0.15 0.5 263] QTE
  ;;[0.15 0.15 0.15 0.5] remove QTE_waiting & call umg
  (Utilities|IsValid (Variables|QTE|GetUMG_QTE_waiting)
    (:Is%20Valid
      (Widget|RemovefromParent (Variables|QTE|GetUMG_QTE_waiting))
      (Development|PrintString "remove done_14455" true true "(R=0.368149,G=0.076611,B=1.000000,A=1.000000)" 5.0)
      (Variables|QTE|SetUMG_QTE_waiting 0))
    (:Is%20Not%20Valid
      (Development|PrintString "umg is not valid(done remove)_14455" true true "(R=0.251143,G=0.000000,B=1.000000,A=1.000000)" 5.0)))
  (Utilities|IsValid (Variables|QTE|GetUMG_call_player_help)
    (:Is%20Valid
      (Widget|RemovefromParent (Variables|QTE|GetUMG_call_player_help)))))

(event Custom|evt_hide_helpUI
  ;[0.15 0.15 0.15 0.5 263] QTE
  ;;[0.15 0.05586 0.02569 0.5] create _call_help umg
  (CallFunction|RemovefromParentinCtrl)
  (Variables|QTE|SetIs%20%20umg%20Valid?%20 false)
  (Variables|QTE|SetUMG_call_player_help 0))

(event Custom|Hide_umg
  (Widget|RemovefromParent (Variables|QTE|GetAs%20QTE%20Switch%20UWG%201)))

(event Custom|Update%20QTE
  (bind _as_qte_switch_uwg_1 (Variables|QTE|GetAs%20QTE%20Switch%20UWG%201))
  (bind _as_gm_play_map (Variables|Default|GetAs%20Gm%20Play%20Map))
  (bind _is_player_done_qte (Variables|/Game/1_text/MP_Framework/game_play_framework/gm_play_map.gm_play_map_C|Getis%20player%20done%20qte _as_gm_play_map))
  (bind _success (Variables|/Game/1_text/MP_Framework/game_play_framework/QTE/QTE_UI/QTE_Switch_UWG.QTE_Switch_UWG_C|GetSuccess _as_qte_switch_uwg_1))
  (Development|PrintString (Utilities|String|ToString(Boolean) _is_player_done_qte) true true "(R=0.447917,G=0.465315,B=1.000000,A=1.000000)")
  (if _is_player_done_qte
    (Utilities|Time|PauseTimerbyHandle (Variables|QTE|Getqte%20TIMER%20handle))
    (Development|PrintString "QTE is done _ 42sdf")
    (UserInterface|Animation|PlayAnimation _as_qte_switch_uwg_1 _success 0.0 1 "Forward" 1.0 false)
    ;[0.15 0.15 0.15 0.5] 為指定的 Widget 動畫綁定一個事件，當該動畫播放結束時，自動觸發你設定的函數
    (Class|UserWidget|BindtoAnimationFinished (Variables|QTE|GetAs%20QTE%20Switch%20UWG%201) _success (delegate Custom|Hide_umg))
    (else
      ;[0.15 0.15 0.15 0.5] 漸漸減少
      (bind (_player_0___no_ _player_1___no_) (Default|QTEUpdatewithNoPowen (Variables|Default|GetAs%20Gm%20Play%20Map) self))
      (CallFunction|CLNUpdateQTE _player_0___no_ _player_1___no_))))

(event Custom|SRV_Notify_otherPlayer
  (params (calling%20help%20controller :type Player%20Controller%20Object%20Reference))
  ;[0.15 0.15 0.15 0.5 263] QTE
  (bind _asgm_play_map (Utilities|Casting|CastTogm_play_map (Game|GetGameMode)))
  ;;[0.15 0.001936 0 0.5] here will call CLN_Receive_other_playerHelp
  (Default|FindOtherPlayer _asgm_play_map calling%20help%20controller "/Game/1_text/MP_Framework/game_play_framework/QTE/QTE_UI/QTE_call_other_player.QTE_call_other_player_C"))

(event Custom|what%20is%20G%20need%20to%20do
  (params (calling%20help%20controller :type Player%20Controller%20Object%20Reference))
  ;[0.15 0.15 0.15 0.5 263] QTE
  ;;[0.15 0.15 0.15 0.5 66] what is G need to do
  (bind _asgm_play_map (Utilities|Casting|CastTogm_play_map (Game|GetGameMode)))
  (if (Utilities|Enum|Equal(Enum) (Variables|/Game/1_text/MP_Framework/game_play_framework/gm_play_map.gm_play_map_C|GetcurrentQTEStste _asgm_play_map) "NewEnumerator0")
    (Development|PrintString "player ctrl : eunm is call none            w5" true true "(R=1.000000,G=0.506122,B=0.241655,A=1.000000)" 5.0)
    (elif (Utilities|Enum|Equal(Enum) (Variables|/Game/1_text/MP_Framework/game_play_framework/gm_play_map.gm_play_map_C|GetcurrentQTEStste _asgm_play_map) "NewEnumerator1")
      (Development|PrintString "player ctrl : eunm is call  waiting  for partner          w5" true true "(R=1.000000,G=0.506122,B=0.241655,A=1.000000)" 5.0)
      (CallFunction|CallOtherPlayer calling%20help%20controller)
      (elif (Utilities|Enum|Equal(Enum) (Variables|/Game/1_text/MP_Framework/game_play_framework/gm_play_map.gm_play_map_C|GetcurrentQTEStste _asgm_play_map) "NewEnumerator2")
        (Development|PrintString "player ctrl : eunm is call  start QTE          w5" true true "(R=1.000000,G=0.506122,B=0.241655,A=1.000000)" 5.0)
        (Variables|QTE|SetQTE%20CurrentEnergy (Math|Float|Clamp(Float) (+ (Variables|QTE|GetQTE%20CurrentEnergy) (Variables|QTE|GetQTE%20ClickPower)) 0.0 1e+02))
        (Default|SERUpdateQte _asgm_play_map self)))))

(event Custom|CLN_Receive_other_playerHelp
  (params (umg%20target :type Self%20Object%20Reference) (UWG :type User%20Widget%20Class%20Reference) (need%20remove%20UI :type Boolean))
  ;[0.15 0.15 0.15 0.5 263] QTE
  ;;[0.15 0.05586 0.02569 0.5] create _call_help umg
  (bind _uiwidget (CallFunction|CreateWidget umg%20target UWG false (Variables|QTE|GetUMG_call_player_help)))
  (bind _output_get (Variables|QTE|SetUMG_call_player_help _uiwidget))
  (Utilities|IsValid _output_get
    (:Is%20Valid
      (Development|PrintString "CLN_Receive_other_playerHelp_        is true235145")
      (Utilities|Time|SetTimerbyEvent (delegate Custom|evt_hide_helpUI) 1.0))
    (:Is%20Not%20Valid
      (Development|PrintString "CLN_Receive_other_playerHelp_        is false235145"))))

(event EventBeginPlay
  ;[0.15 0.02561 0.1444 0.5 50] GAME START SETING
  (if (Pawn|IsLocalPlayerController)
    ;;[0.15 0.15 0.15 0.5] !!!!!!!!!!
    (Input|SetInputModeGameandUI self 0 "DoNotLock" true false)
    (Variables|Default|SetbShowMouseCursor false)
    (Variables|cc_umg|Setis%20ready%20to%20get%20cc false)))

(event EventReadCC
  (params (WhichLine :type Integer) (ShouldContinOutputCC :type Boolean) (HowManyLine :type Integer)))

(event EventQteCatchCtrl
  (params (GM%20ref :type Gm%20Play%20Map%20Object%20Reference))
  ;[0.15 0.15 0.15 0.5 263] QTE
  (Development|PrintString "BPI qte catch ctrl is call ")
  (Utilities|IsValid GM%20ref
    (:Is%20Valid
      (Default|SERWaitingQTE GM%20ref self))
    (:Is%20Not%20Valid
      (Development|PrintString "gm is not valid"))))

(fn ConstructionScript)

(fn CreateWidget
  (params (UWG :type User%20Widget%20Class%20Reference) (need%20set%20boolean? :type Boolean) (umg%20InputObject :type User%20Widget%20Object%20Reference))
  (LocalVariables|SetUMG_create umg%20InputObject)
  (if (not need%20set%20boolean?)
    (Utilities|IsValid (LocalVariables|GetUMG_create)
      (:Is%20Valid
        _)
      (:Is%20Not%20Valid
        (bind _returnvalue (UserInterface|CreateWidget UWG self))
        (LocalVariables|SetUMG_create _returnvalue)))
    (UserInterface|Viewport|AddtoViewport (LocalVariables|GetUMG_create) 0)
    (return (LocalVariables|GetUMG_create))))

(fn QTEFill
  (params (RS%20Target :type Radial%20Slider%20Object%20Reference))
  (Utilities|FlowControl|Sequence
    (:then_0
      (Default|PlayerPulse (Variables|QTE|GetAs%20QTE%20Switch%20UWG%201)))
    (:then_1
      (Variables|QTE|Setplayer_QTE%20Progress (+ (Class|RadialSlider|GetValue RS%20Target) 0.1)))))

(fn ReferencetoSubtitleControl
  (return (Variables|cc_umg|Getumg_cc)))