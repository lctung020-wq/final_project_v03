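; BP_organ_administraator is a manager for rotary puzzle objects, recording which player interacts with which rotary.
; SER_notifyhitplayer stores the hit player, controller, rotary and UMG visibility flag, and clears the original view target.
; The camera switch and return events are empty; blending to the rotary's child-actor camera target, restoring the view and calling the player's input-context function sit in disconnected nodes that never run.
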(event Custom|SER_back%20to%20orignal_cam
  ;[0.0647 0.15 0.1056 0.5 50] rotary  object
)

(event Custom|SER_notify%20hit%20player
  (params (out%20hit%20player%20 :type FPS%20Little%20Brother%20Gv%2002%20Object%20Reference) (out%20hit%20player%20ctrl :type BP%20Player%20Controller%20Text%20Object%20Reference) (hit%20rotary :type Bp%20Rotary%20Refractoir%20Object%20Reference) (UMG%20is%20visibility :type Boolean))
  ;[0.0647 0.15 0.1056 0.5 50] rotary  object
  (Variables|Default|SetOut%20Hit%20Player out%20hit%20player%20)
  ;;[0.15 0.15 0.15 0.5] know which  bp_rotary_refractoir was hit
  (Variables|Default|SetOut%20Hit%20Player%20Ctrl out%20hit%20player%20ctrl)
  (Variables|Default|SetOriginal%20View%20Target 0)
  (Variables|Default|Setrotary%20obj%20UMG%20Is%20Visibility UMG%20is%20visibility)
  (Variables|Default|SetHit%20Rotary hit%20rotary))

(event Custom|CLN_switch_cam
  ;[0.0647 0.15 0.1056 0.5 50] rotary  object
)

(fn ConstructionScript)