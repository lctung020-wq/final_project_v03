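; BP_MoonSlot is a moon-stage puzzle socket that accepts an overlapping BP_PuzzleSelf piece whose PuzzleID matches its MoonPuzzleID.
; On a match, it makes the player drop the piece, snaps it in place, calls the player's ServerDestroyActor to destroy it, and detaches and freezes a StaticMesh.
; It then reports to its parent actor, or increments BP_MoonPuzzleManager progress if none exists.
; Mismatches send only Fire to ServerDestroyActor.
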(event OnComponentBeginOverlap(BoxCollision)
  (params (OverlappedComponent :type Primitive%20Component%20Object%20Reference) (OtherActor :type Actor%20Object%20Reference) (OtherComp :type Primitive%20Component%20Object%20Reference) (OtherBodyIndex :type Integer) (bFromSweep :type Boolean) (SweepResult :type Hit%20Result%20Structure%20%28by%20ref%29))
  (bind _staticmesh (Variables|Default|GetStaticMesh))
  (bind _asbp_puzzle_self (Utilities|Casting|CastToBP_PuzzleSelf OtherActor))
  (Development|PrintString "moon slot is hit puzzle 5z5c")
  (Variables|Default|SetAs%20BP%20Puzzle%20Self _asbp_puzzle_self)
  ;[0.1213 0.07163 0.15 1 30] 改
  (bind _asfps_little_brother_gv_02 (Utilities|Casting|CastToFPS_LittleBrother_Gv02 (Game|GetPlayerCharacter 0)))
  (if (== (Variables|/Game/Superliminal_adeline/Moon_Stage/BP_PuzzleSelf.BP_PuzzleSelf_C|GetPuzzleID _asbp_puzzle_self) (Variables|Default|GetMoon_PuzzleID))
    (Variables|Default|Setpuzzle%20is%20success true)
    (Default|DropObjectG _asfps_little_brother_gv_02)
    (Transformation|SetActorLocationAndRotation _asbp_puzzle_self (Transformation|GetActorLocation) (Transformation|GetActorRotation))
    ;[0.1213 0.07163 0.15 1 30] 改
    (Default|ServerDestroyActor _asfps_little_brother_gv_02 (Variables|Default|GetFire) (Variables|Default|GetStaticMesh) (Variables|Default|GetAs%20BP%20Puzzle%20Self))
    (Variables|Default|SetAs%20BP%20Puzzle%20Self 0)
    ;[0.15 0.15 0.15 0.5] 把一個「附著在別人身上的物件」解鎖並獨立出來。
    (Transformation|DetachFromComponent (Variables|Default|GetStaticMesh) "KeepWorld" "KeepWorld" "KeepWorld" true)
    (Physics|SetSimulatePhysics _staticmesh false)
    (Collision|SetCollisionEnabled _staticmesh "NoCollision")
    (CallFunction|NotifyContainer)
    (else
      (Default|ServerDestroyActor _asfps_little_brother_gv_02 (Variables|Default|GetFire)))))

(event Custom|Server_NotifyContainer
  (params (Target :type Object%20Object%20Reference) (PieceRef :type BP%20Moon%20Slot%20Object%20Reference) (isCompleted :type Boolean))
  (Class|BPIPuzzleContainer|UpdatePuzzleStatus(Message) Target PieceRef isCompleted))

(event EventBeginPlay
  (Rendering|SetVisibility (Variables|Default|GetFire) false false)
  (Rendering|SetVisibility (Variables|Default|GetLandingDecal) false false))

(fn ConstructionScript
  (|CallParentFunction))

(fn NotifyContainer
  (bind _returnvalue (Actor|GetParentActor))
  (Utilities|IsValid _returnvalue
    (:Is%20Valid
      (Development|PrintString (Utilities|GetDisplayName _returnvalue) true true "(R=0.454154,G=1.000000,B=0.348939,A=1.000000)" 1e+01)
      (Class|BPIPuzzleContainer|UpdatePuzzleStatus(Message) _returnvalue self (Variables|Default|Getpuzzle%20is%20success))
      (Development|PrintString "attach parent actor bpi is call    6zcSd"))
    (:Is%20Not%20Valid
      (Development|PrintString "attach parent actor is not valid    6zcSd")
      (bind _returnvalue_2 (Actor|GetActorOfClass "/Game/Superliminal_adeline/Moon_Stage/BP_MoonPuzzleManager.BP_MoonPuzzleManager_C"))
      (Variables|/Game/Superliminal_adeline/Moon_Stage/BP_MoonPuzzleManager.BP_MoonPuzzleManager_C|SetCurrent%20Puzzle%20Fixed _returnvalue_2 (+ (Variables|/Game/Superliminal_adeline/Moon_Stage/BP_MoonPuzzleManager.BP_MoonPuzzleManager_C|GetCurrent%20Puzzle%20Fixed _returnvalue_2) 1))
      (Default|CheckPuzzleProgress _returnvalue_2))))