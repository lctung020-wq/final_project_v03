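; BP_PuzzleSelf is a puzzle object for the Moon Stage that can be picked up and dropped.
; Pickup refuses when the piece is locked; otherwise it snaps the mesh to the supplied component, keeps its world rotation and scale, and stops physics.
; While held, the mesh is query-only, ignoring pawns and overlapping static world.
; Drop detaches it in place, restores physics and blocking collision, and clears the held flag.
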(event EventBeginPlay)

(fn ConstructionScript)

(fn PuzzleSelfDrop
  (bind _staticmesh (Variables|Default|GetStaticMesh))
  (Transformation|DetachFromComponent (Variables|Default|GetStaticMesh) "KeepWorld" "KeepWorld" "KeepWorld" true)
  (Physics|SetSimulatePhysics _staticmesh true)
  (Collision|SetCollisionResponsetoChannel _staticmesh "ECC_Pawn" "ECR_Block")
  (Collision|SetCollisionResponsetoChannel _staticmesh "ECC_WorldStatic" "ECR_Block")
  (Collision|SetCollisionEnabled _staticmesh "QueryAndPhysics")
  (Variables|Default|SetPuzzle_IsHeld false))

(fn PuzzleSelfPickup
  (params (Parent%20Comp :type Scene%20Component%20Object%20Reference))
  (bind _staticmesh (Variables|Default|GetStaticMesh))
  (if (Variables|Default|GetPuzzle_IsLocked)
    (return false)
    (else
      (Transformation|AttachComponentToComponent (Variables|Default|GetStaticMesh) Parent%20Comp "None" "SnapToTarget" "KeepWorld" "KeepWorld" true)
      (Physics|SetSimulatePhysics _staticmesh false)
      (Collision|SetCollisionResponsetoChannel _staticmesh "ECC_Pawn" "ECR_Ignore")
      (Collision|SetCollisionResponsetoChannel _staticmesh "ECC_WorldStatic" "ECR_Overlap")
      (Collision|SetCollisionEnabled _staticmesh "QueryOnly")
      (Variables|Default|SetPuzzle_IsHeld true)
      (return true))))