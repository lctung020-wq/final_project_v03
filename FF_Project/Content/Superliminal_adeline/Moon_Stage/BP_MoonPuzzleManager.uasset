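; Manager for the Moon stage puzzle that also carries a boss-style health pool.
; When the fixed puzzle count reaches the required total, it plays a level sequence once, disabling player 0's input until a timer of about seven seconds restores it.
; A separate damage event clamps health on the authority and forwards it to the gm_play_map game mode to update boss HP.
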(event Custom|Manager_TakeDamage
  (params (DamgeAmount :type Float%20%28double-precision%29) (player%20ctrl :type Controller%20Object%20Reference))
  (Development|PrintString "fps player 1: on hit call 3.5                        sd54g45h")
  (Networking|SwitchHasAuthority
    (:Authority
      (bind _output_get (Variables|Default|SetHealth (Math|Float|Clamp(Float) (- (Variables|Default|GetHealth) DamgeAmount) 0.0 (Variables|Default|GetMaxHealth))))
      (Development|PrintString (Utilities|String|ToString(Float) _output_get))
      (bind _asgm_play_map (Utilities|Casting|CastTogm_play_map (Game|GetGameMode))
        (:then
          (Default|SerBoossHpUpdate _asgm_play_map (Variables|Default|GetMaxHealth) (Variables|Default|GetHealth) player%20ctrl))
        (:CastFailed
          (Development|PrintString "Manager_TakeDamage: cast to failed                         4kmg6fvg4684 "))))))

(event Custom|MoveAgain
  ;[0.15 0.15 0.15 0.5] !!! What will happen
  (Input|EnableInput (Game|GetPlayerCharacter 0) (Game|GetPlayerController 0)))

(event Custom|CheckPuzzleProgress
  (if (>= (Variables|Default|GetCurrent%20Puzzle%20Fixed) (Variables|Default|GetMoon_TotalPuzzleNeed))
    (Utilities|FlowControl|DoOnce false
      (:Completed
        ;[0.15 0.15 0.15 0.5] !!! What will happen
        (Utilities|FlowControl|Sequence
          (:then_0
            (bind _outactor (Sequencer|Player|CreateLevelSequencePlayer 0))
            (Utilities|IsValid _outactor
              (:Is%20Valid
                (Input|DisableInput (Game|GetPlayerCharacter 0) (Game|GetPlayerController 0))
                (Sequencer|Player|Play (Variables|/Script/LevelSequence.LevelSequenceActor|GetSequencePlayer _outactor) :!class /Script/MovieScene.MovieSceneSequencePlayer)
                (Utilities|Time|SetTimerbyEvent (delegate Custom|MoveAgain) 7.03333)
                (Development|PrintString "Hello")))))))))

(fn ConstructionScript)