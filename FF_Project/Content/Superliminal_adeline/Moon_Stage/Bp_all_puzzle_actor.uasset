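; Puzzle container actor for the Moon stage that tracks completed pieces and reports when the whole puzzle is solved.
; BeginPlay passes TotalPiecesNeeded to BP_MoonPuzzleManager, then recalculates it as the child actor component count minus one.
; UpdatePuzzleStatus counts completions.
; When the count matches, it calls SerUpdatPuzzlIsDone on the FPS_LittleBrother_Gv02 actor, passing the PuzzleComplete child actor component, its static mesh and itself.
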(event Custom|puzzle%20is%20done)

(event EventBeginPlay
  (bind _returnvalue (Actor|GetActorOfClass "/Game/Superliminal_adeline/Moon_Stage/BP_MoonPuzzleManager.BP_MoonPuzzleManager_C"))
  (Variables|/Game/Superliminal_adeline/Moon_Stage/BP_MoonPuzzleManager.BP_MoonPuzzleManager_C|SetMoon_TotalPuzzleNeed _returnvalue (Variables|Default|GetTotalPiecesNeeded))
  (Variables|Default|SetTotalPiecesNeeded (- (Utilities|Array|Length (Actor|GetComponentsByClass "/Script/Engine.ChildActorComponent")) 1)))

(event EventUpdatePuzzleStatus
  (params (PieceRef :type BP%20Moon%20Slot%20Object%20Reference) (isCompleted :type Boolean))
  (bind _puzzle_complete (Variables|Default|Getpuzzle_complete))
  (if isCompleted
    (Math|Integer|IncrementInt (Variables|Default|GetCurrentFinishedCount)
      (:%20%20
        (Development|PrintString "BPI updat puzzle is call      a536f4v6ag4fggg" true true "(R=0.132472,G=1.000000,B=0.091655,A=1.000000)")
        (if (== (Variables|Default|GetCurrentFinishedCount) (Variables|Default|GetTotalPiecesNeeded))
          (bind _returnvalue (Actor|GetActorOfClass "/Game/Superliminal_adeline/FPS_LittleBrother_Gv02.FPS_LittleBrother_Gv02_C"))
          (Default|SerUpdatPuzzlIsDone _returnvalue _puzzle_complete (Actor|GetComponentbyClass (Variables|/Script/Engine.ChildActorComponent|GetChildActor _puzzle_complete) "/Script/Engine.StaticMeshComponent") 0 self))))))

(event EventTick
  (params (DeltaSeconds :type Float%20%28single-precision%29)))

(fn ConstructionScript)