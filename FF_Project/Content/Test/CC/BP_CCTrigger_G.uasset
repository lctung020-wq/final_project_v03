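; Test trigger actor that starts closed-caption playback when the third-person character enters its box.
; The first qualifying overlap passes a DoOnce and sends the React message.
; The React event gets the CC object and calls ReadCCMessage for a continued run of lines.
; ReadCC and ReferenceToSubtitleControl are empty, and a sound-at-location call is left unconnected.
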(event OnComponentBeginOverlap(Box)
  (params (OverlappedComponent :type Primitive%20Component%20Object%20Reference) (OtherActor :type Actor%20Object%20Reference) (OtherComp :type Primitive%20Component%20Object%20Reference) (OtherBodyIndex :type Integer) (bFromSweep :type Boolean) (SweepResult :type Hit%20Result%20Structure%20%28by%20ref%29))
  (Utilities|Casting|CastToBP_ThirdPersonCharacter OtherActor)
  (Utilities|FlowControl|DoOnce false
    (:Completed
      (Class|BPIFunctionG|React(Message) self))))

(event EventBeginPlay)

(event Collision|EventActorBeginOverlap
  (params (OtherActor :type Actor%20Object%20Reference)))

(event EventTick
  (params (DeltaSeconds :type Float%20%28single-precision%29)))

(event EventReact
  (Class|BPIFunctionG|ReadCC(Message) (CallFunction|GetCC) 1 true 3))

(event EventReadCC
  (params (WhichLine :type Integer) (ShouldContinOutputCC :type Boolean) (HowManyLine :type Integer)))

(fn ConstructionScript)

(fn ReferencetoSubtitleControl
  (return 0))