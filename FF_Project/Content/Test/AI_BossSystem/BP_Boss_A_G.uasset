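; Networked boss character with parryable melee, a stamina-based stun and tracking pillar attacks, forwarding damage to BP_BossFightManager_G.
; Server-handled melee hits damage each player unless FPS_BigBrother_G parries within range, facing and timing window, which drains boss stamina.
; Empty stamina triggers a timed stun and stand-up, synced to the AI blackboard and brain, with multicast montages.
; A delayed server timer spawns a tracking pillar on every player, but only the last is kept for cancellation.
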(event OnHit(BossMeleeCollisionHandler)
  (params (HitResult :type Hit%20Result%20Structure))
  (bind _returnvalue (Transformation|GetActorLocation))
  (bind _alreadyhitactors (Variables|Default|GetAlreadyHitActors))
  (Networking|SwitchHasAuthority
    (:Authority
      (bind _asbp_first_person_character (Utilities|Casting|CastToBP_FirstPersonCharacter (.HitActor (Collision|BreakHitResult HitResult))))
      (if (not (Utilities|Array|ContainsItem _alreadyhitactors _asbp_first_person_character))
        (Utilities|Array|AddUnique _alreadyhitactors _asbp_first_person_character)
        ;[0.15 0.15 0.15 0.5] 被格擋? Only 哥哥路線
        (bind _asfps_big_brother_g (Utilities|Casting|CastToFPS_BigBrother_G _asbp_first_person_character)
          (:then
            (Variables|Default|SetAs%20FPS%20Big%20Brother%20G _asfps_big_brother_g)
            ;[0.15 0.15 0.15 0.5] ParrySuccess
            (if (Math|Boolean|ANDBoolean (<= (Transformation|GetDistanceTo _asfps_big_brother_g) (Variables|/Game/Superliminal/FPS_BigBrother_G.FPS_BigBrother_G_C|GetParryMaxDistance _asfps_big_brother_g)) (>= (Math|Vector|DotProduct (Math|Vector|Normalize (Math|Vector|MakeVector (- (.x _returnvalue) (.x (Transformation|GetActorLocation _asfps_big_brother_g))) (- (.y _returnvalue) (.y (Transformation|GetActorLocation _asfps_big_brother_g))) 0.0)) (Transformation|GetActorForwardVector _asfps_big_brother_g)) (Variables|/Game/Superliminal/FPS_BigBrother_G.FPS_BigBrother_G_C|GetParryFacingDotMinimun _asfps_big_brother_g)) (Math|Boolean|ANDBoolean (Variables|/Game/Superliminal/FPS_BigBrother_G.FPS_BigBrother_G_C|GetIsParryWindowOpen _asfps_big_brother_g) (Variables|格擋|GetIsAttackParryable) (not (Variables|格擋|GetIsBossStunned)) (not (Variables|格擋|GetParryConsumedThisSwing))))
              (Variables|格擋|SetParryConsumedThisSwing true)
              (Default|DeactivateCollision (Variables|Default|GetBossMeleeCollisionHandler))
              (Default|ConsumeParry (Variables|Default|GetAs%20FPS%20Big%20Brother%20G))
              (CallFunction|BossHandleSuccessfulParry)
              (else
                (Game|Damage|ApplyDamage _asbp_first_person_character (Variables|Default|GetCurrentAttackDamage) (Pawn|GetController) self))))
          (:CastFailed
            ;[0.15 0.15 0.15 0.5] If 是弟弟
            (Game|Damage|ApplyDamage _asbp_first_person_character (Variables|Default|GetCurrentAttackDamage) (Pawn|GetController) self)))))))

(event Custom|MC_PlayAttackVisual
  (params (MontageToPlay :type Anim%20Montage%20Object%20Reference) (WarpTransform :type Transform))
  (Networking|SwitchHasAuthority
    (:Remote
      (Class|MotionWarpingComponent|AddorUpdateWarpTargetfromTransform (Variables|Default|GetMotionWarping) "AttackTarget" WarpTransform)
      (Animation|Montage|MontagePlay (Components|SkeletalMesh|GetAnimInstance (Variables|Character|GetMesh)) MontageToPlay 1.0 "MontageLength" 0.0 true))))

(event Custom|OnBossDeath
  ;[0.4792 0.06489 0.06489 0.5 30] Boss Death
  (Default|DeactivateCollision (Variables|Default|GetBossMeleeCollisionHandler))
  (bind _returnvalue (Animation|PlayAnimMontage 0 1.0 "None"))
  (Utilities|FlowControl|Delay _returnvalue)
  (Actor|DestroyActor)
  (Utilities|IsValid (Variables|Default|GetActiveTrackingPillarAttack)
    (:Is%20Valid
      (Default|ServerCancelAttack (Variables|Default|GetActiveTrackingPillarAttack))
      (Variables|Default|SetActiveTrackingPillarAttack 0))))

(event Custom|BeginBossRecovery
  ;[0.15 0.05654 0.1372 0.5 34] Parry後的各種反應
  (Variables|格擋|SetCurrentBossStamina (Variables|格擋|GetMaxBossStamina))
  (Default|CallOnStaminaChanged (Variables|格擋|GetCurrentBossStamina) (Variables|格擋|GetMaxBossStamina))
  (CallFunction|MCPlayBossStandUp)
  ;;[0.15 0.15 0.15 0.5 42] 起身完成
  (Utilities|Time|SetTimerbyEvent (delegate Custom|FinishBossRecovery) (Variables|格擋|GetBossStandUpDuration)))

(event Custom|FinishBossRecovery
  ;[0.15 0.05654 0.1372 0.5 34] Parry後的各種反應
  ;;[0.15 0.15 0.15 0.5 42] 起身完成
  (Variables|格擋|SetIsBossStunned false)
  (Pawn|Components|CharacterMovement|SetMovementMode (Variables|Character|GetCharacterMovement) "MOVE_Walking" 0)
  (AI|Components|Blackboard|SetValueasBool (AI|GetBlackboard (AI|GetAIController self)) (Utilities|String|StringToName "IsBossStunned") false)
  (Class|BrainComponent|RestartLogic (Variables|/Script/AIModule.AIController|GetBrainComponent (AI|GetAIController self))))

(event Custom|StartTrackingPillarAttack
  ;[0.2287 0.6979 0.1738 0.5 30] 生成攻擊 Actor
  ;;[0.15 0.15 0.15 0.5 25] For BTT_MeleeCombo - 遠程攻擊的最終完整節點
  (Networking|SwitchHasAuthority
    (:Authority
      (if (not (Variables|格擋|GetIsBossStunned))
        (Utilities|Time|SetTimerbyEvent (delegate Custom|Server_SpawnTrackingPillarTimer) (Variables|施法關鍵動作需時|GetTrackingPillarSpawnDelay))))))

(event Custom|MC_PlayRangedAttackMontage
  ;[0.2287 0.6979 0.1738 0.5 30] 生成攻擊 Actor
  ;;[0.15 0.15 0.15 0.5] Useless
  (Animation|Montage|PlayMontage (Variables|Character|GetMesh) "/Game/Test/Animation_Test/NewMontage_G/Boss/AM_Boss_Long-RangeAttack_v1_G.AM_Boss_Long-RangeAttack_v1_G"))

(event Custom|Server_SpawnTrackingPillarTimer
  (bind _self self)
  ;[0.2287 0.6979 0.1738 0.5 30] 生成攻擊 Actor
  ;;[0.15 0.15 0.15 0.5] Only提醒自己：
  ;; 這是一段只能由 Server 執行的 Gameplay Logic, 不需要設定成 Run on Server RPC
  (Networking|SwitchHasAuthority
    (:Authority
      (bind _outactors (Actor|GetAllActorsOfClass "/Game/FirstPerson/Blueprints/BP_FirstPersonCharacter.BP_FirstPersonCharacter_C"))
      (Variables|Default|SetMultiTargetActor _outactors)
      (for _array_element _outactors
        (Utilities|IsValid _array_element
          (:Is%20Valid
            (bind _returnvalue (Game|SpawnActorfromClass "/Game/Test/AI_BossSystem/LongRangeAttack/BP_BossTrackingPillarAttack_G.BP_BossTrackingPillarAttack_G_C" (Math|Transform|MakeTransform (Transformation|GetActorLocation _array_element)) "Undefined" "MultiplyWithRoot" _self _array_element _self))
            (bind _output_get (Variables|Default|SetActiveTrackingPillarAttack _returnvalue))
            (Variables|/Game/Test/AI_BossSystem/LongRangeAttack/BP_BossTrackingPillarAttack_G.BP_BossTrackingPillarAttack_G_C|SetOwningBoss _output_get self)
            (Default|ServerInitializeAttack (Variables|Default|GetActiveTrackingPillarAttack))))))))

(event Custom|Boss_HandleSuccessfulParry
  ;[0.15 0.08276 0.04612 0.5 40] 成功Parry後的判斷
  (if (not (Variables|格擋|GetIsBossStunned))
    (Variables|格擋|SetCurrentBossStamina (Math|Float|Clamp(Float) (- (Variables|格擋|GetCurrentBossStamina) (Variables|格擋|GetParryStaminaDamage)) 0.0 (Variables|格擋|GetMaxBossStamina)))
    (Default|CallOnStaminaChanged (Variables|格擋|GetCurrentBossStamina) (Variables|格擋|GetMaxBossStamina))
    (Development|PrintString (Utilities|String|ToString(Float) (Variables|格擋|GetCurrentBossStamina)))
    (if (<= (Variables|格擋|GetCurrentBossStamina) 0.0)
      (CallFunction|EnterBossStunned)
      (else
        (CallFunction|MCPlayBossParryReact)))))

(event Custom|EnterBossStunned
  (bind _self self)
  (bind _activetrackingpillarattack (Variables|Default|GetActiveTrackingPillarAttack))
  (bind _returnvalue (AI|GetAIController _self))
  ;[0.15 0.05654 0.1372 0.5 34] Parry後的各種反應
  (if (not (Variables|格擋|GetIsBossStunned))
    (Utilities|IsValid _activetrackingpillarattack
      (:Is%20Valid
        (Default|ServerCancelAttack _activetrackingpillarattack))
      (:Is%20Not%20Valid
        _))
    (Variables|格擋|SetIsBossStunned true)
    (Variables|格擋|SetCurrentBossStamina 0.0)
    (Default|CallOnStaminaChanged (Variables|格擋|GetCurrentBossStamina) (Variables|格擋|GetMaxBossStamina))
    (Variables|格擋|SetIsAttackParryable false)
    (Variables|格擋|SetParryConsumedThisSwing true)
    (Default|DeactivateCollision (Variables|Default|GetBossMeleeCollisionHandler))
    (AI|Navigation|StopMovement _returnvalue)
    (AI|Components|Blackboard|SetValueasBool (AI|GetBlackboard _returnvalue) (Utilities|String|StringToName "IsBossStunned") true)
    (CallFunction|MCPlayBossStunEnter)
    (Utilities|Time|SetTimerbyEvent (delegate Custom|BeginBossRecovery) (Variables|格擋|GetBossStunDuration))))

(event Custom|MC_PlayBossParryReact
  ;[0.15 0.05654 0.1372 0.5 34] Parry後的各種反應
  ;;[0.15 0.15 0.15 0.5 30] 普通被格擋
  (Animation|Montage|PlayMontage (Variables|Character|GetMesh) "/Game/Test/Animation_Test/NewMontage_G/Boss/AM_BossAnim_GetParried_G.AM_BossAnim_GetParried_G"))

(event Custom|MC_PlayBossStandUp
  (bind _self self)
  (bind _charactermovement (Variables|Character|GetCharacterMovement))
  (bind _returnvalue (AI|GetAIController _self))
  (bind _braincomponent (Variables|/Script/AIModule.AIController|GetBrainComponent _returnvalue))
  ;[0.15 0.05654 0.1372 0.5 34] Parry後的各種反應
  ;;[0.15 0.15 0.15 0.5 34] StandUp
  (Components|Movement|StopMovementImmediately _charactermovement)
  (Pawn|Components|CharacterMovement|SetMovementMode _charactermovement "MOVE_None" 0)
  (AI|Logic|StopLogic _braincomponent "Stun")
  (Animation|Montage|PlayMontage 0 "/Game/Test/Animation_Test/NewMontage_G/Boss/AM_BossAnim_GetUp_G.AM_BossAnim_GetUp_G"
    (:OnCompleted
      _)
    (:OnInterrupted
      _))
  (Pawn|Components|CharacterMovement|SetMovementMode _charactermovement "MOVE_Walking" 0)
  (Class|BrainComponent|RestartLogic _braincomponent))

(event Custom|Server_BeginBossParryReact
  (bind _self self)
  (bind _returnvalue (AI|GetAIController _self))
  ;[0.15 0.05654 0.1372 0.5 34] Parry後的各種反應
  ;;[0.15 0.15 0.15 0.5 30] 伺服器事件 - 普通格擋反應狀態
  (Default|DeactivateCollision (Variables|Default|GetBossMeleeCollisionHandler))
  (Variables|格擋|SetIsAttackParryable false)
  (AI|Navigation|StopMovement _returnvalue)
  (AI|Components|Blackboard|SetValueasBool (AI|GetBlackboard _returnvalue) (Utilities|Name|MakeLiteralName "IsBossParryReacting") true)
  (CallFunction|MCPlayBossParryReact)
  (Utilities|Time|SetTimerbyEvent (delegate Custom|Server_EndBossParryReact) 0.68))

(event Custom|Server_EndBossParryReact
  ;[0.15 0.05654 0.1372 0.5 34] Parry後的各種反應
  ;;[0.15 0.15 0.15 0.5 30] 伺服器事件 - 普通格擋反應狀態
  (AI|Components|Blackboard|SetValueasBool (AI|GetBlackboard (AI|GetAIController self)) (Utilities|Name|MakeLiteralName "IsBossParryReacting") false))

(event Custom|MC_PlayBossStunEnter
  ;[0.15 0.05654 0.1372 0.5 34] Parry後的各種反應
  ;;[0.15 0.15 0.15 0.5 26] 暈倒
  (Animation|Montage|PlayMontage (Variables|Character|GetMesh) "/Game/Test/Animation_Test/NewMontage_G/Boss/AM_BossAnim_Exhuastion_Loop_G.AM_BossAnim_Exhuastion_Loop_G"))

(event Game|Damage|EventAnyDamage
  (params (Damage :type Float%20%28single-precision%29) (DamageType :type Damage%20Type%20Object%20Reference) (InstigatedBy :type Controller%20Object%20Reference) (DamageCauser :type Actor%20Object%20Reference))
  (Default|DeactivateCollision (Variables|Default|GetBossMeleeCollisionHandler))
  (bind _returnvalue (Actor|GetActorOfClass "/Game/Test/BP_BossFightManager_G.BP_BossFightManager_G_C"))
  (Default|ManagerTakeDamage _returnvalue Damage)
  (Animation|PlayAnimMontage "/Game/Test/Animation_Test/NewMontage_G/Boss/AM_BossAnim_GetHit_G.AM_BossAnim_GetHit_G" 1.0 "None"))

(event EventBeginPlay
  (Networking|SwitchHasAuthority
    (:Authority
      (bind _collidingcomponents (CallFunction|ConvertPrimitivetoCollidingComponent (Variables|Default|GetWeapon) "Trace_"))
      (Variables|/Game/DynamicCombatSystem/DCS/Blueprints/Components/CollisionHandler/BP_CollisionHandlerComponent.BP_CollisionHandlerComponent_C|SetCollisionComponents (Variables|Default|GetBossMeleeCollisionHandler) (Utilities|Array|MakeArray _collidingcomponents))
      (Variables|格擋|SetCurrentBossStamina (Variables|格擋|GetMaxBossStamina))
      (Default|CallOnStaminaChanged (Variables|格擋|GetCurrentBossStamina) (Variables|格擋|GetMaxBossStamina)))))

(fn ConstructionScript)

(fn OnRepIsBossStunned)

(fn OnRepCurrentBossStamina
  (Default|CallOnStaminaChanged (Variables|格擋|GetCurrentBossStamina) (Variables|格擋|GetMaxBossStamina)))

(fn ClearTrackingPillarReference
  (Variables|Default|SetActiveTrackingPillarAttack 0))