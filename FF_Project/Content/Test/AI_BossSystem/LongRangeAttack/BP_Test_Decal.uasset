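; Test Blueprint for a long-range attack telegraph, sizing a danger-area decal and a shrinking warning-ring decal.
; UpdateDecalSizes converts radii to Y/Z decal scales relative to a base diameter, with an extra multiplier for the danger area.
; Tick currently passes a fixed ring radius.
; Disconnected logic interpolates the ring from start radius to attack radius using server time across tracking and lock durations.
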(event EventTick
  (params (DeltaSeconds :type Float%20%28single-precision%29))
  (CallFunction|UpdateDecalSizes 1e+02))

(event EventBeginPlay)

(fn ConstructionScript)

(fn UpdateDecalSizes
  (params (CurrentWarningRadius :type Float%20%28double-precision%29))
  ;[0.15 0.15 0.15 0.5 30] Decal_DangerArea 危險圈本身大小
  (bind _output_get (LocalVariables|SetAttackDiameter (* (Variables|Default|GetAttackRadius) 2.0)))
  (LocalVariables|SetDangerScale (* (/ _output_get (Variables|Default|GetBaseDecalDiameter)) (LocalVariables|GetDangerDecalScaleMultiplier)))
  (Transformation|SetRelativeScale3D (Variables|Default|GetDecal_DangerArea) (Math|Vector|MakeVector 1.0 (LocalVariables|GetDangerScale) (LocalVariables|GetDangerScale)))
  ;[0.15 0.15 0.15 0.5 22] Decal_ShrinkingRing :
  ; 把縮圈 Decal 的實際直徑，從 WarningStartRadius 到目前的 CurrentWarningRadius
  (bind _output_get_2 (LocalVariables|SetWarningDiameter (* CurrentWarningRadius 2.0)))
  (LocalVariables|SetRingScale (/ _output_get_2 (Variables|Default|GetBaseDecalDiameter)))
  (Transformation|SetRelativeScale3D (Variables|Default|GetDecal_ShrinkingRing) (Math|Vector|MakeVector 1.0 (LocalVariables|GetRingScale) (LocalVariables|GetRingScale))))