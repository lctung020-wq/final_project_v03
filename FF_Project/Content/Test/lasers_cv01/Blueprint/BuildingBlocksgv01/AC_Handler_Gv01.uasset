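; Actor component that acts as the laser-hit hub for its owning actor in a laser building-block system.
; On BeginPlay it gathers sibling laser-interface components, sets static meshes to block a trace channel, and, if inverted, calls stop-hitting on emitters.
; It tracks incoming lasers and relays hit start/stop unless locked, updates on authority, and conditional forced activation/deactivation.
; Start, stop and forced changes then call the activate or deactivate handler.
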(event EventBeginPlay
  (Utilities|FlowControl|Sequence
    (:then_0
      (bind _output_get (Variables|Default|SetLinked%20Components (Class|Actor|GetComponentsbyInterface (Components|GetOwner) "/Game/Test/lasers_cv01/Blueprint/BuildingBlocksgv01/BPI_Lasers_Gv01.BPI_Lasers_Gv01_C")))
      (Utilities|Array|RemoveItem _output_get self)
      (for _array_element (Actor|GetComponentsByClass (Components|GetOwner) "/Script/Engine.StaticMeshComponent")
        (Collision|SetCollisionResponsetoChannel _array_element "ECC_GameTraceChannel3" (select (Variables|Conditions|GetIsBlocking) "ECR_Block" "ECR_Block"))))
    (:then_1
      (if (Variables|Conditions|GetInvert%20System)
        (for _array_element_2 (Actor|GetComponentsByClass (Components|GetOwner) "/Game/Test/lasers_cv01/Blueprint/BuildingBlocksgv01/SC_Emitter_Gv01.SC_Emitter_Gv01_C")
          (Default|LaserStopHitting _array_element_2))))))

(event EventLaserUpdateHitting
  (params (Input :type A%20Laser%20Gv%2001%20Object%20Reference) (Hit%20Info :type Hit%20Result%20Structure))
  (Networking|SwitchHasAuthority
    (:Authority
      (bind _array_element (Utilities|ForEachComponent)
        (:LoopBody
          (Class|BPILasersGv01|LaserUpdateHitting(Message) _array_element Input Hit%20Info))))))

(event EventForceActivation
  (params (ApplyConditions :type Boolean))
  (if ApplyConditions
    (if (Variables|Default|GetIsHit)
      (bind _array_element (Utilities|ForEachComponent)
        (:LoopBody
          (Class|BPILasersGv01|ForceActivation(Message) _array_element ApplyConditions))
        (:Completed
          (Default|CallActivateHandler self))))))

(event EventLaserStartHitting
  (params (Input :type A%20Laser%20Gv%2001%20Object%20Reference) (Hit%20Info :type Hit%20Result%20Structure))
  (CallFunction|LaserAdded Input)
  (Utilities|IsNotLocked
    (:Not%20Locked
      (bind _array_element (Utilities|ForEachComponent)
        (:LoopBody
          (Class|BPILasersGv01|LaserStartHitting(Message) _array_element Input Hit%20Info))
        (:Completed
          (Default|CallActivateHandler self))))))

(event EventLaserStopHitting
  (params (Input :type A%20Laser%20Gv%2001%20Object%20Reference))
  (CallFunction|LaserRemove Input)
  (Utilities|IsNotLocked
    (:Not%20Locked
      (bind _array_element (Utilities|ForEachComponent)
        (:LoopBody
          (Class|BPILasersGv01|LaserStopHitting(Message) _array_element Input))
        (:Completed
          (Default|CallDeactivateHandler self))))))

(event EventForceDeactivation
  (params (ApplyConditions :type Boolean))
  (if ApplyConditions
    (if (not (Variables|Default|GetIsHit))
      (bind _array_element (Utilities|ForEachComponent)
        (:LoopBody
          (Class|BPILasersGv01|ForceDeactivation(Message) _array_element ApplyConditions))
        (:Completed
          (Default|CallDeactivateHandler self))))))

(fn LaserAdded
  (params (NewItem :type A%20Laser%20Gv%2001%20Object%20Reference%20%28by%20ref%29))
  (Utilities|Array|AddUnique (Variables|Default|GetLasersInQueue) NewItem))

(fn LaserRemove
  (params (NewItem :type A%20Laser%20Gv%2001%20Object%20Reference%20%28by%20ref%29))
  (Utilities|Array|RemoveItem (Variables|Default|GetLasersInQueue) NewItem))

(fn AreAllCompsActivated
  (for _array_element (Variables|Default|GetLinkedExternalComps)
    _))