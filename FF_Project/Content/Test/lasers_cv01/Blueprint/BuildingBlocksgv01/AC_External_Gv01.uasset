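; Actor component that links its owner to AC_Handler_Gv01 components on target actors, relaying activate and deactivate signals for mechanism triggers.
; By default it binds to each handler and maps its state, seeded from InvertSystem, broadcasting activation only when all are active and deactivation when any deactivates.
; With InvertControl it instead registers itself in each handler's linked list, binds external events, and broadcasts changes directly without the all-active check.
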(event Custom|tex)

(event EventBeginPlay
  ;[0.15 0.15 0.15 0.5] If Turn on Bottom?
  (if (Variables|Default|GetInvertControl)
    (for _array_element (Variables|Default|GetTargetActors)
      (Utilities|IsValid (Actor|GetComponentbyClass _array_element "/Game/Test/lasers_cv01/Blueprint/BuildingBlocksgv01/AC_Handler_Gv01.AC_Handler_Gv01_C")
        (:Is%20Valid
          (Utilities|Array|AddUnique (Variables|/Game/Test/lasers_cv01/Blueprint/BuildingBlocksgv01/AC_Handler_Gv01.AC_Handler_Gv01_C|GetLinkedExternalComps (Actor|GetComponentbyClass _array_element "/Game/Test/lasers_cv01/Blueprint/BuildingBlocksgv01/AC_Handler_Gv01.AC_Handler_Gv01_C")) self)
          (EventDispatchers|BindEventtoExternalActivate (EventDispatchers|CreateEvent (Actor|GetComponentbyClass _array_element "/Game/Test/lasers_cv01/Blueprint/BuildingBlocksgv01/AC_Handler_Gv01.AC_Handler_Gv01_C") :!event ForceActivation))
          (EventDispatchers|BindEventtoExternalDeactivate (EventDispatchers|CreateEvent (Actor|GetComponentbyClass _array_element "/Game/Test/lasers_cv01/Blueprint/BuildingBlocksgv01/AC_Handler_Gv01.AC_Handler_Gv01_C") :!event ForceDeactivation)))))
    (else
      ;[0.15 0.15 0.15 0.5] Main: 機關觸發
      (for _array_element_2 (Variables|Default|GetTargetActors)
        (Utilities|IsValid (Actor|GetComponentbyClass _array_element_2 "/Game/Test/lasers_cv01/Blueprint/BuildingBlocksgv01/AC_Handler_Gv01.AC_Handler_Gv01_C")
          (:Is%20Valid
            (Utilities|Map|Add (Variables|Default|GetNeceesaryActors) (Actor|GetComponentbyClass _array_element_2 "/Game/Test/lasers_cv01/Blueprint/BuildingBlocksgv01/AC_Handler_Gv01.AC_Handler_Gv01_C") (Variables|/Game/Test/lasers_cv01/Blueprint/BuildingBlocksgv01/AC_Handler_Gv01.AC_Handler_Gv01_C|GetInvert%20System (Actor|GetComponentbyClass _array_element_2 "/Game/Test/lasers_cv01/Blueprint/BuildingBlocksgv01/AC_Handler_Gv01.AC_Handler_Gv01_C")))
            (EventDispatchers|BindEventtoActivateHandler (Actor|GetComponentbyClass _array_element_2 "/Game/Test/lasers_cv01/Blueprint/BuildingBlocksgv01/AC_Handler_Gv01.AC_Handler_Gv01_C") (EventDispatchers|CreateEvent :!event ActivateThis))
            (EventDispatchers|BindEventtoDeactivateHandler (Actor|GetComponentbyClass _array_element_2 "/Game/Test/lasers_cv01/Blueprint/BuildingBlocksgv01/AC_Handler_Gv01.AC_Handler_Gv01_C") (EventDispatchers|CreateEvent :!event DeactivateThis))))))))

(fn ActivateThis
  (params (Instigator :type AC%20Handler%20Gv%2001%20Object%20Reference))
  (if (Variables|Default|GetInvertControl)
    (Variables|Default|SetIsComActivated true)
    (Default|CallExternalActivate (Variables|Default|GetApplyConditions))
    (else
      (Utilities|FlowControl|Sequence
        (:then_0
          (Utilities|Map|Add (Variables|Default|GetNeceesaryActors) Instigator true))
        (:then_1
          (if (CallFunction|AllActorsActive)
            (Default|CallExternalActivate (Variables|Default|GetApplyConditions))))))))

(fn DeactivateThis
  (params (Instigator :type AC%20Handler%20Gv%2001%20Object%20Reference))
  (if (Variables|Default|GetInvertControl)
    (Variables|Default|SetIsComActivated false)
    (Default|CallExternalDeactivate (Variables|Default|GetApplyConditions))
    (else
      (Utilities|Map|Add (Variables|Default|GetNeceesaryActors) Instigator false)
      (Default|CallExternalDeactivate (Variables|Default|GetApplyConditions)))))

(fn AllActorsActive
  (bind _keys (Utilities|Map|Keys (Variables|Default|GetNeceesaryActors)))
  (for _array_element _keys
    (if (not (.Value (Utilities|Map|Find (Variables|Default|GetNeceesaryActors) _array_element)))
      (return false)))
  (return true))