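; BP_BossFightManager_G manages a boss fight by holding one health pool for the BP_Boss_A_G and BP_Boss_B_G bosses.
; Manager_TakeDamage subtracts incoming damage and clamps Health between zero and MaxHealth.
; At zero, it finds every actor of both boss classes and destroys them.
; Unconnected OnBossDeath calls are left as a noted alternative to DestroyActor for bosses with unique death events.
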(event Custom|Manager_TakeDamage
  (params (DamgeAmount :type Float%20%28double-precision%29))
  (Variables|Default|SetHealth (Math|Float|Clamp(Float) (- (Variables|Default|GetHealth) DamgeAmount) 0.0 (Variables|Default|GetMaxHealth)))
  (if (<= (Variables|Default|GetHealth) 0.0)
    (bind _outactors (Actor|GetAllActorsOfClass "/Game/Test/AI_BossSystem/BP_Boss_A_G.BP_Boss_A_G_C"))
    (for _array_element _outactors
      (Actor|DestroyActor _array_element))
    (bind _outactors_2 (Actor|GetAllActorsOfClass "/Game/Test/BP_Boss_B_G.BP_Boss_B_G_C"))
    (for _array_element_2 _outactors_2
      (Actor|DestroyActor _array_element_2))))

(fn ConstructionScript)