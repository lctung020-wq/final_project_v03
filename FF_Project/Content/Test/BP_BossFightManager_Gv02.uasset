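; Boss fight manager Blueprint that tracks a boss's health when it takes damage.
; Its server damage event, guarded by an authority check, subtracts the amount and clamps health between zero and the maximum.
; It then passes the new and max health, with the attacking player controller, to the gm_play_map game mode for an HP update.
; Boss death calls are present but unconnected, and debug prints trace the flow.
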(event Custom|SER_Manager_TakeDamage
  (params (DamgeAmount :type Float%20%28double-precision%29) (player%20ctrl :type Controller%20Object%20Reference))
  (Development|PrintString "fps player 1: on hit call 3.5                        sd54g45h")
  (Networking|SwitchHasAuthority
    (:Authority
      (bind _output_get (Variables|Default|SetHealth (Math|Float|Clamp(Float) (- (Variables|Default|GetHealth) DamgeAmount) 0.0 (Variables|Default|GetMaxHealth))))
      (Development|PrintString (Utilities|String|ToString(Float) _output_get) true true "(R=1.000000,G=0.210392,B=0.987317,A=1.000000)")
      ;[0.1213 0.07163 0.15 1 30] 改
      (bind _asgm_play_map (Utilities|Casting|CastTogm_play_map (Game|GetGameMode))
        (:then
          (Default|SerBoossHpUpdate _asgm_play_map (Variables|Default|GetMaxHealth) (Variables|Default|GetHealth) player%20ctrl)
          (Development|PrintString "fps player 1: on hit call 4                         sd54g45h"))
        (:CastFailed
          (Development|PrintString "Manager_TakeDamage: gm cast to failed                         4kmg6fvg4684 " true true "(R=1.000000,G=0.015401,B=0.000000,A=1.000000)"))))))

(fn ConstructionScript)