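; Boss ranged attack actor that follows a target player's ground position with a shrinking warning ring, then erupts as a damaging Niagara pillar.
; Server timers and delays drive an AttackState through tracking, locked and impact to finished or cancelled, with OnRep refreshing visuals.
; Gated Tick scales the decals from server world time and keeps tracing the actor under the target, even when locked.
; Impact damage uses a sphere overlap narrowed by a cylinder test around the locked location.
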(event Custom|Server_InitializeAttack
  (Networking|SwitchHasAuthority
    (:Authority
      (Utilities|IsValid (Variables|參考變數|GetTargetActor)
        (:Is%20Valid
          (Variables|本機與伺服器變數|SetDamageResolved false)
          (Variables|網絡狀態|SetAttackState "NewEnumerator1")
          (CallFunction|ApplyVisualState)
          (Networking|ForceNetUpdate)
          (Variables|網絡狀態|SetAttackStartServerTime (GameState|GetServerWorldTimeSeconds (Game|GetGameState)))
          (CallFunction|ServerUpdateTrackingLocation)
          (bind _returnvalue (Utilities|Time|SetTimerbyEvent (delegate Custom|Server_UpdateTrackingLocation) (Variables|時間與範圍|GetTrackingUpdateRate) true))
          (Variables|本機與伺服器變數|SetTrackingTimerHandle _returnvalue)
          (Utilities|Time|SetTimerbyEvent (delegate Custom|Server_LockAttackLocation) (Variables|時間與範圍|GetTrackingDuration)))))))

(event Custom|Server_UpdateTrackingLocation
  (bind _targetactor (Variables|參考變數|GetTargetActor))
  (bind _targetactor_2 (Variables|參考變數|GetTargetActor))
  (bind _returnvalue (Transformation|GetActorLocation _targetactor))
  ;[0.15 0.15 0.15 0.5] 持續Tracking 伺服器同步 : 玩家在哪裡？-> 玩家腳下的地面在哪裡？
  (Networking|SwitchHasAuthority
    (:Authority
      (if (Utilities|Enum|Equal(Enum) (Variables|網絡狀態|GetAttackState) "NewEnumerator1")
        (Utilities|IsValid _targetactor_2
          (:Is%20Valid
            (Variables|Default|SetActors%20to%20Ignore (Utilities|Array|MakeArray _targetactor_2))
            (CallFunction|CEStartWarning)
            (bind (_outhit _returnvalue_2) (Collision|LineTraceByChannel (+ _returnvalue "0.000000,0.000000,1000.000000") (- _returnvalue "0.000000,0.000000,2000.000000") "TraceTypeQuery4" false (Variables|Default|GetActors%20to%20Ignore) "None"))
            (if _returnvalue_2
              (Transformation|SetActorLocation (+ (.ImpactPoint (Collision|BreakHitResult _outhit)) (* (.ImpactNormal (Collision|BreakHitResult _outhit)) (Variables|Default|GetGroundOffset))) false false)
              (else
                (CallFunction|ServerCancelAttack)))))))))

(event Custom|Server_LockAttackLocation
  (Networking|SwitchHasAuthority
    (:Authority
      (Development|PrintString "Run Server_LockAttackLocation" true true "(R=0.084088,G=0.000000,B=1.000000,A=1.000000)")
      (Utilities|Time|ClearandInvalidateTimerbyHandle (Variables|本機與伺服器變數|GetTrackingTimerHandle))
      (Variables|網絡狀態|SetLockedGroundLocation (Transformation|GetActorLocation))
      (Variables|網絡狀態|SetAttackState "NewEnumerator2")
      (CallFunction|ApplyVisualState)
      (Networking|ForceNetUpdate)
      (Utilities|Time|SetTimerbyEvent (delegate Custom|Server_ResolveImpact) 0.0))))

(event Custom|Server_CancelAttack
  ;[0.5417 0.07271 0.06193 0.5 30] 取消
  (Networking|SwitchHasAuthority
    (:Authority
      (if (and (Utilities|Enum|NotEqual(Enum) (Variables|網絡狀態|GetAttackState) "NewEnumerator5") (Utilities|Enum|NotEqual(Enum) (Variables|網絡狀態|GetAttackState) "NewEnumerator4"))
        (Utilities|Time|ClearandInvalidateTimerbyHandle (Variables|本機與伺服器變數|GetTrackingTimerHandle))
        (Utilities|Time|ClearandInvalidateTimerbyHandle (Variables|本機與伺服器變數|GetImpactTimerHandle))
        (Variables|本機與伺服器變數|SetDamageResolved false)
        (Variables|網絡狀態|SetAttackState "NewEnumerator4")
        (CallFunction|ApplyVisualState)
        (Networking|ForceNetUpdate)
        (Utilities|FlowControl|Delay 0.1)
        (Actor|DestroyActor)))))

(event Custom|Server_ResolveImpact
  (Networking|SwitchHasAuthority
    (:Authority
      (Development|PrintString "Run Server_ResolveImpact")
      (if (== (Variables|本機與伺服器變數|GetDamageResolved) false)
        (Variables|本機與伺服器變數|SetDamageResolved true)
        (Variables|網絡狀態|SetAttackState "NewEnumerator3")
        (CallFunction|CEStopWarning)
        (CallFunction|ApplyVisualState)
        (Networking|ForceNetUpdate)
        (Variables|Default|SetDamageCenter (+ (Variables|網絡狀態|GetLockedGroundLocation) (Math|Vector|MakeVector 0.0 0.0 (Variables|時間與範圍|GetCylinderHalfHeight))))
        (Variables|Default|SetSearchRadius (Math|Float|Sqrt (+ (* (Variables|時間與範圍|GetAttackRadius) (Variables|時間與範圍|GetAttackRadius)) (* (Variables|時間與範圍|GetCylinderHalfHeight) (Variables|時間與範圍|GetCylinderHalfHeight)))))
        (bind _outactors (Collision|SphereOverlapActors (Variables|Default|GetDamageCenter) (Variables|Default|GetSearchRadius) (Variables|Default|GetPawn) "/Game/FirstPerson/Blueprints/BP_FirstPersonCharacter.BP_FirstPersonCharacter_C" (Utilities|Array|MakeArray (Variables|參考變數|GetOwningBoss))))
        ;[0.15 0.15 0.15 0.5] 對每名玩家做真正的圓柱判定
        (for _array_element _outactors
          (Variables|Default|SetPlayerLocation (Transformation|GetActorLocation _array_element))
          (Variables|Default|SetDelta (- (Variables|Default|GetPlayerLocation) (Variables|Default|GetDamageCenter)))
          (Variables|Default|SetHorizontalDistanceSquared (+ (* (.x (Variables|Default|GetDelta)) (.x (Variables|Default|GetDelta))) (* (.y (Variables|Default|GetDelta)) (.y (Variables|Default|GetDelta)))))
          (Variables|技能圓柱判定|SetInsideHorizontal (<= (Variables|Default|GetHorizontalDistanceSquared) (* (Variables|時間與範圍|GetAttackRadius) (Variables|時間與範圍|GetAttackRadius))))
          (Variables|技能圓柱判定|SetInsideVertical (<= (Math|Float|Absolute(Float) (.z (Variables|Default|GetDelta))) (Variables|時間與範圍|GetCylinderHalfHeight)))
          (Variables|技能圓柱判定|SetInsideCylinder (and (Variables|技能圓柱判定|GetInsideHorizontal) (Variables|技能圓柱判定|GetInsideVertical)))
          (if (Variables|技能圓柱判定|GetInsideCylinder)
            (Game|Damage|ApplyDamage (Utilities|Array|Get(acopy) (Variables|Default|GetDamaged%20Actor)) (Variables|時間與範圍|GetAttackDamage) (Game|GetInstigatorController) (Variables|參考變數|GetOwningBoss))
            (Utilities|Time|SetTimerbyEvent (delegate Custom|Server_FinishAttack) (Variables|時間與範圍|GetCleanupDuration))))))))

(event Custom|Server_FinishAttack
  (bind _owningboss (Variables|參考變數|GetOwningBoss))
  (Variables|網絡狀態|SetAttackState "NewEnumerator5")
  (CallFunction|ApplyVisualState)
  (Actor|DestroyActor)
  (Utilities|IsValid _owningboss
    (:Is%20Valid
      (Default|ClearTrackingPillarReference _owningboss))))

(event Custom|CE_StopWarning
  (bind _targetactor (Variables|參考變數|GetTargetActor))
  (bind _returnvalue (Transformation|GetActorLocation _targetactor))
  ;[0.3532 0.839 1 0.5 30] 本機更新縮圈動畫
  (CallFunction|ApplyVisualState)
  (Networking|ForceNetUpdate)
  (Utilities|FlowControl|Gate true) ; enters at Close
)

(event Custom|CE_StartWarning
  (bind _targetactor (Variables|參考變數|GetTargetActor))
  (bind _returnvalue (Transformation|GetActorLocation _targetactor))
  ;[0.3532 0.839 1 0.5 30] 本機更新縮圈動畫
  (Utilities|FlowControl|Sequence
    (:then_0
      (CallFunction|ApplyVisualState)
      (Networking|ForceNetUpdate)
      (Utilities|FlowControl|Gate true) ; enters at Open
    )
    (:then_1
      (Utilities|FlowControl|Delay (+ (Variables|時間與範圍|GetTrackingDuration) (Variables|時間與範圍|GetLockDuration)))
      (CallFunction|CEStopWarning)
      (CallFunction|ServerResolveImpact))))

(event EventTick
  (params (DeltaSeconds :type Float%20%28single-precision%29))
  (bind _targetactor (Variables|參考變數|GetTargetActor))
  (bind _returnvalue (Transformation|GetActorLocation _targetactor))
  ;[0.3532 0.839 1 0.5 30] 本機更新縮圈動畫
  (Utilities|FlowControl|Gate true
    (:Exit
      (if (or (Utilities|Enum|Equal(Enum) (Variables|網絡狀態|GetAttackState) "NewEnumerator1") (Utilities|Enum|Equal(Enum) (Variables|網絡狀態|GetAttackState) "NewEnumerator2"))
        (Variables|Default|SetCurrentServerTime (GameState|GetServerWorldTimeSeconds (Game|GetGameState)))
        (Variables|外圈|SetTotalTelegraphDuration (+ (Variables|時間與範圍|GetTrackingDuration) (Variables|時間與範圍|GetLockDuration)))
        (Variables|外圈|SetProgress (Math|Float|MapRangeClamped (Variables|Default|GetCurrentServerTime) (Variables|網絡狀態|GetAttackStartServerTime) (+ (Variables|網絡狀態|GetAttackStartServerTime) (Variables|外圈|GetTotalTelegraphDuration)) 0.0 1.0))
        ;;[0.004132 0.3801 1 0.5] 目前外圈半徑
        (Variables|外圈|SetCurrentWarningRadius (Math|Float|Lerp (Variables|時間與範圍|GetWarningStartRadius) (* (Variables|時間與範圍|GetAttackRadius) (Variables|實際危險圓比例|GetDangerDecalScaleMultiplier)) (Variables|外圈|GetProgress)))
        (CallFunction|UpdateDecalSizes (Variables|外圈|GetCurrentWarningRadius))
        ;;[0.1042 0.1042 0.1042] 把 BP_BossTrackingPillarAttack 移到那裡
        (bind (_outhit _returnvalue_2) (Collision|LineTraceByChannel (+ _returnvalue "0.000000,0.000000,1000.000000") (- _returnvalue "0.000000,0.000000,2000.000000") "TraceTypeQuery4" false (Variables|Default|GetActors%20to%20Ignore) "ForDuration"))
        (if _returnvalue_2
          (Transformation|SetActorLocation (+ (.ImpactPoint (Collision|BreakHitResult _outhit)) (* (.ImpactNormal (Collision|BreakHitResult _outhit)) (Variables|Default|GetGroundOffset))) false false)
          (else
            (CallFunction|ServerCancelAttack)))))))

(fn ConstructionScript)

(fn OnRepAttackState
  (CallFunction|ApplyVisualState)
  (Components|Activation|Activate (Variables|Default|GetNiagara_PillarImpact) true))

(fn UpdateDecalSizes
  (params (CurrentWarningRadius :type Float%20%28double-precision%29))
  ;[0.15 0.15 0.15 0.5 30] Decal_DangerArea 危險圈本身大小
  (bind _output_get (LocalVariables|SetAttackDiameter (* (Variables|時間與範圍|GetAttackRadius) 2.0)))
  (LocalVariables|SetDangerScale (* (/ _output_get (Variables|Default|GetBaseDecalDiameter)) (Variables|實際危險圓比例|GetDangerDecalScaleMultiplier)))
  (Transformation|SetRelativeScale3D (Variables|Default|GetDecal_DangerArea) (Math|Vector|MakeVector 1.0 (LocalVariables|GetDangerScale) (LocalVariables|GetDangerScale)))
  ;[0.15 0.15 0.15 0.5 22] Decal_ShrinkingRing :
  ; 把縮圈 Decal 的實際直徑，從 WarningStartRadius 到目前的 CurrentWarningRadius
  (bind _output_get_2 (LocalVariables|SetWarningDiameter (* CurrentWarningRadius 2.0)))
  (LocalVariables|SetRingScale (/ _output_get_2 (Variables|Default|GetBaseDecalDiameter)))
  (Transformation|SetRelativeScale3D (Variables|Default|GetDecal_ShrinkingRing) (Math|Vector|MakeVector 1.0 (LocalVariables|GetRingScale) (LocalVariables|GetRingScale))))

(fn ApplyVisualState
  (bind _niagara_pillarimpact (Variables|Default|GetNiagara_PillarImpact))
  (switch Utilities|FlowControl|Switch|SwitchonE_TrackingPillarState (Variables|網絡狀態|GetAttackState)
    (:NewEnumerator1
      (Rendering|SetVisibility (Variables|Default|GetDecal_DangerArea) true false)
      (Rendering|SetVisibility (Variables|Default|GetDecal_ShrinkingRing) true false)
      (Components|Activation|Deactivate (Variables|Default|GetNiagara_PillarImpact)))
    (:NewEnumerator2
      (Rendering|SetVisibility (Variables|Default|GetDecal_DangerArea) true false)
      (Rendering|SetVisibility (Variables|Default|GetDecal_ShrinkingRing) true false)
      (Components|Activation|Deactivate (Variables|Default|GetNiagara_PillarImpact)))
    (:NewEnumerator3
      (Rendering|SetVisibility (Variables|Default|GetDecal_DangerArea) false false)
      (Rendering|SetVisibility (Variables|Default|GetDecal_ShrinkingRing) false false)
      (Niagara|SetNiagaraVariable(Float) _niagara_pillarimpact "User.AttackRadius" (Variables|時間與範圍|GetAttackRadius))
      (Niagara|SetNiagaraVariable(Float) _niagara_pillarimpact "User.PillarHeight" (* (Variables|時間與範圍|GetCylinderHalfHeight) 2.0))
      (Components|Activation|Activate _niagara_pillarimpact true))
    (:NewEnumerator4
      (Rendering|SetVisibility (Variables|Default|GetDecal_DangerArea) false false :!label _label)
      (Rendering|SetVisibility (Variables|Default|GetDecal_ShrinkingRing) false false)
      (Components|Activation|Deactivate (Variables|Default|GetNiagara_PillarImpact)))
    (:NewEnumerator5
      (goto _label))))