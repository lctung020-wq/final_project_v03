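; Rotary refractor level mechanism with a yaw-rotating base and a roll-tilting mirror, adjustable in multiplayer.
; Box overlap toggles its widget, switches lights and reports the player, controller and actor to BP_organ_administraator.
; AuthorityAddRotation sets replicated rotation deltas, which it and the OnReps apply through fixed-step RInterpTo.
; Mirror roll clamps around its BeginPlay angle, playing controller force feedback at either limit.
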(event OnComponentBeginOverlap(Box)
  (params (OverlappedComponent :type Primitive%20Component%20Object%20Reference) (OtherActor :type Actor%20Object%20Reference) (OtherComp :type Primitive%20Component%20Object%20Reference) (OtherBodyIndex :type Integer) (bFromSweep :type Boolean) (SweepResult :type Hit%20Result%20Structure%20%28by%20ref%29))
  (Rendering|SetVisibility (Variables|Default|GetPointLight) true false)
  (bind _asfps_little_brother_gv_02 (Utilities|Casting|CastToFPS_LittleBrother_Gv02 OtherActor))
  (bind _asbp_player_controller_text (Utilities|Casting|CastToBP_player_controller_text (Pawn|GetController _asfps_little_brother_gv_02)))
  (Variables|Default|SetAs%20BP%20Player%20Controller%20Text _asbp_player_controller_text)
  (bind _output_get (Variables|Default|SetUMG%20is%20visibility true))
  (Rendering|SetVisibility (Variables|Default|GetWidget) _output_get false)
  (bind _as_bp_organ_administraator (Variables|Default|GetAS%20BP_organ_administraator)
    (:then
      (Default|SERNotifyHitPlayer _as_bp_organ_administraator _asfps_little_brother_gv_02 _asbp_player_controller_text self (Variables|Default|GetUMG%20is%20visibility)))
    (:else
      (Development|PrintString "AS BP_organ_administraator is not valid                56fh14jdfgch5"))))

(event OnComponentEndOverlap(Box)
  (params (OverlappedComponent :type Primitive%20Component%20Object%20Reference) (OtherActor :type Actor%20Object%20Reference) (OtherComp :type Primitive%20Component%20Object%20Reference) (OtherBodyIndex :type Integer))
  (Utilities|Casting|CastToCharacter OtherActor)
  (bind _output_get (Variables|Default|SetUMG%20is%20visibility false))
  (Rendering|SetVisibility (Variables|Default|GetWidget) _output_get false)
  (bind _as_bp_organ_administraator (Variables|Default|GetAS%20BP_organ_administraator)
    (:then
      (Default|SERNotifyHitPlayer _as_bp_organ_administraator 0 0 0 false)
      (Rendering|SetVisibility (Variables|Default|GetSpotLight) false false))
    (:else)))

(event Custom|notft%20all%20player)

(event EventBeginPlay
  (bind _returnvalue (Actor|GetActorOfClass "/Game/1_text/MP_Framework/game_play_framework/BP_organ_administraator.BP_organ_administraator_C"))
  (Variables|Default|SetAS%20BP_organ_administraator _returnvalue)
  ;[0.15 0.15 0.15 0.5] show widget or not
  (Rendering|SetVisibility (Variables|Default|GetWidget) (Variables|Default|GetUMG%20is%20visibility) false)
  (Variables|Default|Setmirror%20lnital%20angle%20Return%20%20X%20 (.roll (Transformation|GetWorldRotation (Variables|Default|Getmirror%20ChildActor))))
  (Rendering|SetVisibility (Variables|Default|GetSpotLight) false false))

(event Collision|EventActorBeginOverlap
  (params (OtherActor :type Actor%20Object%20Reference)))

(event EventTick
  (params (DeltaSeconds :type Float%20%28single-precision%29)))

(fn ConstructionScript
  (Transformation|SetRelativeTransform (Variables|Default|GetOverviewCamera) (Variables|Default|GetOverviewCameraTransform) false false)
  (Transformation|SetWorldRotation (Variables|Default|GetSTM_rotary) (Math|Rotator|MakeRotator 0.0 0.0 (Variables|Default|GetSTM_rotary%20New%20Transform)) false false))

(fn AuthorityAddRotation
  (params (STM%20RotationDelta :type Float%20%28double-precision%29) (%20Mirror%20RotationDelta :type Float%20%28double-precision%29))
  (if (Variables|Default|GetIs%20not%20Move)
    (Variables|Default|SetMirror%20Rotation%20Delta %20Mirror%20RotationDelta)
    (Variables|Default|SetReplicatedRotationYaw STM%20RotationDelta)
    (STMrotary|ApplyVisualRotation)
    (STMrotary|ApplyVisualRotationMirror)
    (else
      (Variables|Default|SetMirror%20Rotation%20Delta %20Mirror%20RotationDelta)
      (STMrotary|ApplyVisualRotationMirror))))

(fn ApplyVisualRotation
  (bind _stm_rotary (Variables|Default|GetSTM_rotary))
  (bind _is_not_move (Variables|Default|GetIs%20not%20Move))
  (bind _relativerotation (Variables|/Script/Engine.SceneComponent|GetRelativeRotation _stm_rotary))
  (Development|PrintString (Utilities|String|ToString(Boolean) _is_not_move) true true "(R=1.000000,G=0.941545,B=0.000000,A=1.000000)")
  (if _is_not_move
    (Development|PrintString "Hello")
    (bind _output_get (Variables|Default|Setnow%20stm%20angle%20Z%20%28Yaw%29 (.yaw (Math|Interpolation|RInterpTo (Math|Rotator|MakeRotator 0.0 0.0 (.yaw _relativerotation)) (Math|Rotator|MakeRotator 0.0 0.0 (+ (.yaw _relativerotation) (Variables|Default|GetReplicatedRotationYaw))) 0.016 3e+01))))
    (Transformation|SetRelativeRotation (Variables|Default|GetSTM_rotary) (Math|Rotator|MakeRotator 0.0 0.0 _output_get) false false)))

(fn OnRepReplicatedRotationYaw
  (Variables|Default|SetIs%20not%20Move true)
  (STMrotary|ApplyVisualRotation))

(fn OnRepMirrorRotationDelta
  (Variables|Default|SetIs%20not%20Move false)
  (STMrotary|ApplyVisualRotationMirror))

(fn ApplyVisualRotationMirror
  (bind _mirror_childactor (Variables|Default|Getmirror%20ChildActor))
  (bind _returnvalue (Transformation|GetWorldRotation _mirror_childactor))
  (LocalVariables|Setmin%20mirror (+ (Variables|Default|Getmirror%20lnital%20angle%20Return%20%20X%20) -4e+01))
  (LocalVariables|Setmax%20mirror (+ (Variables|Default|Getmirror%20lnital%20angle%20Return%20%20X%20) 6e+01))
  (Transformation|SetRelativeRotation (Variables|Default|Getmirror%20ChildActor) (Math|Rotator|MakeRotator (Math|Float|Clamp(Float) (.roll (Math|Interpolation|RInterpTo (Math|Rotator|MakeRotator (.roll _returnvalue) 0.0 0.0) (Math|Rotator|MakeRotator (Variables|Default|GetMirror%20Rotation%20Delta) 0.0 0.0) 0.016 3e+01)) (LocalVariables|Getmin%20mirror) (LocalVariables|Getmax%20mirror)) 0.0 0.0) false false)
  (if (or (== (.roll _returnvalue) (LocalVariables|Getmin%20mirror)) (== (LocalVariables|Getmax%20mirror) (.roll _returnvalue)))
    (bind _as_bp_player_controller_text (Variables|Default|GetAs%20BP%20Player%20Controller%20Text)
      (:then
        (Game|Feedback|ClientPlayForceFeedback _as_bp_player_controller_text "/Game/Superliminal_adeline/Input/FFE_object_is_max.FFE_object_is_max" "None" false false false))
      (:else))))