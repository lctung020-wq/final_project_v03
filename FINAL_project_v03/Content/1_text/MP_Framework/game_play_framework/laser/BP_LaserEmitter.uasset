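; BP_LaserEmitter is a laser emitter actor that detects hits on actors whose first tag is "Receiver".
; Every Tick, CalculateLaserPath repeats the same Visibility line trace in a loop, from LaserCylinderG along the actor's up vector out to Range, ignoring itself.
; Receiver hit locations are appended to TracePoints, with no clearing or reflection step.
; Persistent debug lines and printed hit names expose each trace.
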(event Custom|CalculateLaserPath
  (bind _laser_cylinder_g (Variables|Default|GetLaser_Cylinder_G))
  (bind _actors_to_ignore (Variables|Default|GetActors%20to%20Ignore))
  (bind _returnvalue (Transformation|GetWorldLocation _laser_cylinder_g))
  (for _index (range 0 10)
    (Utilities|Array|Add _actors_to_ignore self)
    (bind (_outhit _returnvalue_2) (Collision|LineTraceByChannel _returnvalue (+ _returnvalue (* (Transformation|GetActorUpVector) (Variables|Default|GetRange))) "TraceTypeQuery1" false _actors_to_ignore "Persistent"))
    (Development|PrintString (Utilities|GetDisplayName (.HitActor (Collision|BreakHitResult _outhit))))
    (if _returnvalue_2
      (if (== (Utilities|Array|Get(acopy) (Variables|/Script/Engine.Actor|GetTags (.HitActor (Collision|BreakHitResult _outhit)))) "Receiver")
        (Utilities|Array|Add (Variables|Default|GetTracePoints) (.Location (Collision|BreakHitResult _outhit)))))))

(event EventBeginPlay)

(event Collision|EventActorBeginOverlap
  (params (OtherActor :type Actor%20Object%20Reference)))

(event EventTick
  (params (DeltaSeconds :type Float%20%28single-precision%29))
  (CallFunction|CalculateLaserPath))

(fn ConstructionScript)