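; Game mode for the two-player play map, spawning the first login as BigBrother and later ones as LittleBrother at named player starts.
; It relays boss health and QTE state to both players' controllers, fetched by index, through client-prefixed calls.
; For the co-op QTE, it waits on a timeout for two triggering controllers, starts QTE UI on both, mirrors their energy and removes the UI when both are full.
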(event Custom|SER_waiting_QTE
  (params (Qte_triger%20controller :type BP%20Player%20Controller%20Text%20Object%20Reference))
  (bind _all_qte_triger_controller (Variables|Default|Getall_Qte%20Triger%20Controller))
  (bind _returnvalue (Utilities|Array|Length _all_qte_triger_controller))
  (bind _returnvalue_2 (== _returnvalue 2))
  ;[0 0.1477 0.15 0.5 111] QTE
  ;;[0 0.0515 0.15 0.5 20] 觸發QTE:      -當 QTE 事件被觸發時，系統會設定玩家控制器、更新 QTE 狀態，並啟動一個 5 秒的倒數計時器；若時間到玩家未操作，則重置狀態。
  (Development|PrintString "SRV_waiting_QTE has called      true 354gh" true true "(R=1.000000,G=0.000000,B=0.041751,A=1.000000)" 5.0)
  (bind _output_get (Variables|Default|SetQte_triger%20controller Qte_triger%20controller))
  (Utilities|Array|Add (Variables|Default|Getall_Qte%20Triger%20Controller) _output_get)
  (Development|PrintString (Utilities|String|Append "all_Qte Triger Controller" (Utilities|String|ToString(Boolean) _returnvalue_2)) true true "(R=0.000000,G=0.063337,B=1.000000,A=1.000000)")
  (if _returnvalue_2
    (Utilities|Time|ClearandInvalidateTimerbyHandle (Variables|Default|Getwaiting%20all%20player%20_timerHandle))
    ;;;[1 0 0] get two player here
    (Development|PrintString "all player in call       true 354gh" true true "(R=1.000000,G=0.000000,B=0.041751,A=1.000000)" 5.0)
    (CallFunction|SERSetUpQTE (Variables|Default|GetQte_triger%20controller))
    (else
      (Development|PrintString "all player in call      false 354gh" true true "(R=1.000000,G=0.000000,B=0.041751,A=1.000000)" 5.0)
      (Variables|Default|SetcurrentQTEStste "NewEnumerator1")
      ;;;[1 0.01273 0 0.5] this is the timer
      (bind _returnvalue_3 (Utilities|Time|SetTimerbyEvent (delegate Custom|Evt_QTE_timeout) 2e+01))
      (Variables|Default|Setwaiting%20all%20player%20_timerHandle _returnvalue_3)
      (Default|CLNShowWaitingUI (Variables|Default|GetQte_triger%20controller) false)
      (Development|PrintString "Hello"))))

(event Custom|Evt_QTE_timeout
  ;[0 0.1477 0.15 0.5 111] QTE
  ;;[0 0.0515 0.15 0.5 20] 觸發QTE:      -當 QTE 事件被觸發時，系統會設定玩家控制器、更新 QTE 狀態，並啟動一個 5 秒的倒數計時器；若時間到玩家未操作，則重置狀態。
  (Variables|Default|SetcurrentQTEStste "NewEnumerator0")
  (CallFunction|RemoveAllUmgFindOtherPlayer (Variables|Default|GetQte_triger%20controller)))

(event Custom|SER%20Booss%20Hp%20Update
  (params (max%20hp :type Float%20%28double-precision%29) (Hp :type Float%20%28double-precision%29) (player%20ctrl :type Controller%20Object%20Reference))
  (bind _returnvalue (Game|GetPlayerController 0))
  ;[0.15 0.1342 0 0.5 93] Boss hp
  (Development|PrintString "gm : ser_booss hp update is call         5bzd41hsz")
  (Utilities|IsValid _returnvalue
    (:Is%20Valid
      (bind _asbp_player_controller_text (Utilities|Casting|CastToBP_player_controller_text _returnvalue))
      (Development|PrintString (Utilities|String|ToString(Float) Hp) true true "(R=0.000000,G=1.000000,B=0.066711,A=1.000000)"))
    (:Is%20Not%20Valid
      (Development|PrintString "gm : boss hp player 0 not find         5bzd41hsz")))
  (Default|CLNUpdathp _asbp_player_controller_text max%20hp Hp)
  (bind _asbp_player_controller_text_2 (Utilities|Casting|CastToBP_player_controller_text (Game|GetPlayerController 1))
    (:then
      (Default|CLNUpdathp _asbp_player_controller_text_2 max%20hp Hp)
      (Development|PrintString "fps player 1: on hit call 5                           sd54g45h"))
    (:CastFailed
      (Development|PrintString "gm : boss hp player 1 not find         5bzd41hsz"))))

(event Custom|SER_setUpQTE
  (params (sender%20controller :type Player%20Controller%20Object%20Reference))
  ;[0 0.1477 0.15 0.5 111] QTE
  ;;[0 0.0515 0.15 0.5 20] 觸發QTE:      -當 QTE 事件被觸發時，系統會設定玩家控制器、更新 QTE 狀態，並啟動一個 5 秒的倒數計時器；若時間到玩家未操作，則重置狀態。
  (bind _asbp_player_controller_text (Utilities|Casting|CastToBP_player_controller_text sender%20controller))
  (CallFunction|RemoveAllUmgFindOtherPlayer sender%20controller)
  (Utilities|IsValid (Variables|/Game/1_text/MP_Framework/game_play_framework/BP_player_controller_text.BP_player_controller_text_C|GetUMG_QTE_waiting _asbp_player_controller_text)
    (:Is%20Valid
      (CallFunction|SERSetUpQTE _asbp_player_controller_text))
    (:Is%20Not%20Valid
      (Variables|Default|SetcurrentQTEStste "NewEnumerator2")
      (Utilities|FlowControl|Delay 0.2)
      (bind (__player_controller_0 __player_controller_1) (CallFunction|FindOtherPlayer(justPlayer)))
      (Default|CLNCreatStartQTE __player_controller_0 __player_controller_0)
      (Utilities|IsValid __player_controller_1
        (:Is%20Valid
          (Default|CLNCreatStartQTE __player_controller_1 __player_controller_1))))))

(event Custom|SER_update%20qte
  (params (Sender%20ctrl :type Player%20Controller%20Object%20Reference))
  ;[0 0.1477 0.15 0.5 111] QTE
  (bind (__player_controller_0 __player_controller_1) (CallFunction|FindOtherPlayer(justPlayer)))
  (Default|CNLUpdatQte __player_controller_0 (/ (Variables|/Game/1_text/MP_Framework/game_play_framework/BP_player_controller_text.BP_player_controller_text_C|GetQTE%20CurrentEnergy __player_controller_0) 1e+02) (/ (Variables|/Game/1_text/MP_Framework/game_play_framework/BP_player_controller_text.BP_player_controller_text_C|GetQTE%20CurrentEnergy __player_controller_1) 1e+02))
  (Default|CNLUpdatQte __player_controller_1 (/ (Variables|/Game/1_text/MP_Framework/game_play_framework/BP_player_controller_text.BP_player_controller_text_C|GetQTE%20CurrentEnergy __player_controller_0) 1e+02) (/ (Variables|/Game/1_text/MP_Framework/game_play_framework/BP_player_controller_text.BP_player_controller_text_C|GetQTE%20CurrentEnergy __player_controller_1) 1e+02))
  (if (and (== (/ (Variables|/Game/1_text/MP_Framework/game_play_framework/BP_player_controller_text.BP_player_controller_text_C|GetQTE%20CurrentEnergy __player_controller_0) 1e+02) 1.0) (== (/ (Variables|/Game/1_text/MP_Framework/game_play_framework/BP_player_controller_text.BP_player_controller_text_C|GetQTE%20CurrentEnergy __player_controller_1) 1e+02) 1.0))
    (CallFunction|QTEIsDone)))

(event Custom|QTE%20is%20done
  ;[0 0.1477 0.15 0.5 111] QTE
  (bind (__player_controller_0 __player_controller_1) (CallFunction|FindOtherPlayer(justPlayer)))
  (Utilities|FlowControl|Delay 0.5)
  (Default|RemoveQTESwitchUmg __player_controller_0)
  (Default|RemoveQTESwitchUmg __player_controller_1))

(event EventPostLogin
  (params (NewPlayer :type Player%20Controller%20Object%20Reference))
  (bind _returnvalue (Class|GameModeBase|FindPlayerStart NewPlayer "Spawn_playerB"))
  (bind _returnvalue_2 (Class|GameModeBase|FindPlayerStart NewPlayer "Spawn_playerA"))
  (bind _returnvalue_3 (Transformation|GetActorTransform _returnvalue_2))
  (bind _returnvalue_4 (Transformation|GetActorTransform _returnvalue))
  ;[0.15 0.002201 0 0.5 80] player begin spawn
  (if (== (Variables|Default|GetNumPlayer%20Connected) 0)
    (bind _returnvalue_5 (Game|SpawnActorfromClass "/Game/Superliminal_adeline/FPS_BigBrother_Gv02.FPS_BigBrother_Gv02_C" (Math|Transform|MakeTransform (.location _returnvalue_3) (.rotation _returnvalue_3) "1.000000,1.000000,1.000000") "AlwaysSpawn" "MultiplyWithRoot" 0 0))
    (Pawn|Possess NewPlayer _returnvalue_5)
    (Math|Integer|IncrementInt (Variables|Default|GetNumPlayer%20Connected)
      (:%20%20
        _))
    (else
      (bind _returnvalue_6 (Game|SpawnActorfromClass "/Game/Superliminal_adeline/FPS_LittleBrother_Gv02.FPS_LittleBrother_Gv02_C" (Math|Transform|MakeTransform (.location _returnvalue_4) (.rotation _returnvalue_4) "1.000000,1.000000,1.000000") "AlwaysSpawn" "MultiplyWithRoot" 0 7.0 0))
      (Pawn|Possess NewPlayer _returnvalue_6)
      (Math|Integer|IncrementInt (Variables|Default|GetNumPlayer%20Connected)
        (:%20%20
          _))))
  (Development|PrintString (Utilities|String|Append "get player ctrl" (Utilities|String|ToString(Integer) (Variables|Default|GetNumPlayer%20Connected)))))

(fn ConstructionScript)

(fn FindOtherPlayer
  (params (sender%20controller :type Player%20Controller%20Object%20Reference) (UWG1 :type User%20Widget%20Class%20Reference))
  (if (== sender%20controller (Game|GetPlayerController 0))
    (Development|PrintString "is player0")
    (bind _asbp_player_controller_text (Utilities|Casting|CastToBP_player_controller_text (Game|GetPlayerController 1))
      (:then
        (Default|CLNReceiveOtherPlayerHelp _asbp_player_controller_text _asbp_player_controller_text UWG1 false))
      (:CastFailed
        (Development|PrintString "Funcations_find_other_player1 cast failed")))
    (else
      (Development|PrintString "is not player0")
      (bind _asbp_player_controller_text_2 (Utilities|Casting|CastToBP_player_controller_text (Game|GetPlayerController 0))
        (:then
          (Default|CLNReceiveOtherPlayerHelp _asbp_player_controller_text_2 _asbp_player_controller_text_2 UWG1 false))
        (:CastFailed
          (Development|PrintString "Funcations_find_other_player0 cast failed"))))))

(fn RemoveAllUmgFindOtherPlayer
  (params (sender%20controller :type Player%20Controller%20Object%20Reference))
  (bind _asbp_player_controller_text (Utilities|Casting|CastToBP_player_controller_text (Game|GetPlayerController 1)))
  (LocalVariables|Setplayer%20ctrl%201 _asbp_player_controller_text)
  (bind _asbp_player_controller_text_2 (Utilities|Casting|CastToBP_player_controller_text (Game|GetPlayerController 0)))
  (LocalVariables|Setplayer%20ctrl%200 _asbp_player_controller_text_2)
  (if (== sender%20controller (Game|GetPlayerController 0))
    (Development|PrintString "is player0")
    (Default|RemovefromParentinCtrl (LocalVariables|Getplayer%20ctrl%201))
    (Default|RemovefromParentinCtrl (LocalVariables|Getplayer%20ctrl%201))
    (Development|PrintString "Funcationsis done")
    (else
      (Development|PrintString "is not player0")
      (Default|RemovefromParentinCtrl (LocalVariables|Getplayer%20ctrl%200))
      (Default|RemovefromParentinCtrl (LocalVariables|Getplayer%20ctrl%200))
      (Development|PrintString "Funcationsis done"))))

(fn UpdateQteFillPlayer
  (bind _asbp_player_controller_text (Utilities|Casting|CastToBP_player_controller_text (Game|GetPlayerController 1))
    (:then
      ;[0.15 0.15 0.15 0.5] find teo player progress
      (bind _output_get (LocalVariables|Setplayer%201%20ctrl_f_update _asbp_player_controller_text))
      (Default|CLNUpdateQTE _output_get (Variables|/Game/1_text/MP_Framework/game_play_framework/BP_player_controller_text.BP_player_controller_text_C|Getplayer_QTE%20Progress (LocalVariables|Getplayer%200%20ctrl_f_update)) (Variables|/Game/1_text/MP_Framework/game_play_framework/BP_player_controller_text.BP_player_controller_text_C|Getplayer_QTE%20Progress (LocalVariables|Getplayer%201%20ctrl_f_update)))
      (bind _asbp_player_controller_text_2 (Utilities|Casting|CastToBP_player_controller_text (Game|GetPlayerController 0))
        (:then
          (bind _output_get_2 (LocalVariables|Setplayer%200%20ctrl_f_update _asbp_player_controller_text_2))
          (Default|CLNUpdateQTE _output_get_2 (Variables|/Game/1_text/MP_Framework/game_play_framework/BP_player_controller_text.BP_player_controller_text_C|Getplayer_QTE%20Progress (LocalVariables|Getplayer%200%20ctrl_f_update)) (Variables|/Game/1_text/MP_Framework/game_play_framework/BP_player_controller_text.BP_player_controller_text_C|Getplayer_QTE%20Progress (LocalVariables|Getplayer%201%20ctrl_f_update)))
          (Development|PrintString "all player have setting the fil        68r4yw   ")
          (if (and (< (Variables|/Game/1_text/MP_Framework/game_play_framework/BP_player_controller_text.BP_player_controller_text_C|Getplayer_QTE%20Progress (LocalVariables|Getplayer%201%20ctrl_f_update)) 0.56) (< (Variables|/Game/1_text/MP_Framework/game_play_framework/BP_player_controller_text.BP_player_controller_text_C|Getplayer_QTE%20Progress (LocalVariables|Getplayer%200%20ctrl_f_update)) 0.56))
            (Development|PrintString "ALL PLAYER is ready false qte       cvsxfd9+85")
            (Variables|fun_updateqte|Setis%20player%20done%20qte false)
            (else
              (Development|PrintString "ALL PLAYER is ready done qte       cvsxfd9+85" true true "(R=1.000000,G=0.279370,B=0.000000,A=1.000000)" 4.0)
              (Variables|fun_updateqte|Setis%20player%20done%20qte true)))
          (return (Variables|fun_updateqte|Getis%20player%20done%20qte)))
        (:CastFailed
          (Development|PrintString "update qte fill : get plater 0 is failed          azef85354" true true "(R=1.000000,G=0.017847,B=0.000000,A=1.000000)"))))
    (:CastFailed
      (Development|PrintString "update qte fill : get plater 1 is failed          azef85354" true true "(R=1.000000,G=0.017847,B=0.000000,A=1.000000)"))))

(fn QTEUpdatewithNoPowen
  (params (player%20ctrl :type BP%20Player%20Controller%20Text%20Object%20Reference))
  ;[0.15 0 0.006049 0.99 186] !!!!!!!!
  (if (== player%20ctrl (Game|GetPlayerController 0))
    (Development|PrintString "is player0")
    (bind _asbp_player_controller_text (Utilities|Casting|CastToBP_player_controller_text (Game|GetPlayerController 0)))
    (bind _output_get (Variables|/Game/1_text/MP_Framework/game_play_framework/BP_player_controller_text.BP_player_controller_text_C|Setplayer_QTE%20Progress _asbp_player_controller_text (- (Class|RadialSlider|GetValue (Variables|/Game/1_text/MP_Framework/game_play_framework/QTE/QTE_UI/QTE_Switch_UWG.QTE_Switch_UWG_C|GetRS_QTE_player1 (Variables|/Game/1_text/MP_Framework/game_play_framework/BP_player_controller_text.BP_player_controller_text_C|GetAs%20QTE%20Switch%20UWG%201 _asbp_player_controller_text))) (Math|Float|Clamp(Float) (* (Variables|fun_updateqte|GetDecayPerSecond) 0.1)))))
    (else
      (Development|PrintString "is not player0")
      (bind _asbp_player_controller_text_2 (Utilities|Casting|CastToBP_player_controller_text (Game|GetPlayerController 1)))
      (bind _output_get_2 (Variables|/Game/1_text/MP_Framework/game_play_framework/BP_player_controller_text.BP_player_controller_text_C|Setplayer_QTE%20Progress _asbp_player_controller_text_2 (- (Class|RadialSlider|GetValue (Variables|/Game/1_text/MP_Framework/game_play_framework/QTE/QTE_UI/QTE_Switch_UWG.QTE_Switch_UWG_C|GetRS_QTE_player2 (Variables|/Game/1_text/MP_Framework/game_play_framework/BP_player_controller_text.BP_player_controller_text_C|GetAs%20QTE%20Switch%20UWG%201 _asbp_player_controller_text_2))) (Math|Float|Clamp(Float) (* (Variables|fun_updateqte|GetDecayPerSecond) 0.1)))))))
  (fun_updateqte|UpdateQteFillPlayer)
  (return _output_get _output_get_2))

(fn FindOtherPlayer(justPlayer)
  (bind _asbp_player_controller_text (Utilities|Casting|CastToBP_player_controller_text (Game|GetPlayerController 0))
    (:then
      (bind _asbp_player_controller_text_2 (Utilities|Casting|CastToBP_player_controller_text (Game|GetPlayerController 1))
        (:then
          (return _asbp_player_controller_text _asbp_player_controller_text_2))
        (:CastFailed
          (Development|PrintString "Funcations_find_other_player1 cast failed"))))
    (:CastFailed
      (Development|PrintString "Funcations_find_other_player0 cast failed"))))

(fn ReferencetoSubtitleControl
  (return 0))